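; Mountain ape AI character that damages others through punch, slam and body contact while moving.
; Animation notify events open and close trace windows; Tick sweeps the left hand for punches and both hands for slams, tracking hit actors.
; Closing a slam window also applies radial damage below the AoEChecker.
; The DamageVolume applies passive knockback damage on overlap when X speed is high enough; roar handlers only cast the anim instance.
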(event OnComponentBeginOverlap(DamageVolume)
  (params (OverlappedComponent :type Primitive%20Component%20Object%20Reference) (OtherActor :type Actor%20Object%20Reference) (OtherComp :type Primitive%20Component%20Object%20Reference) (OtherBodyIndex :type Integer) (bFromSweep :type Boolean) (SweepResult :type Hit%20Result%20Structure%20%28by%20ref%29))
  (bind _returnvalue (Transformation|GetActorLocation))
  (bind _returnvalue_2 (Transformation|GetActorLocation OtherActor))
  ;[1 1 1] Apply damage to playes getting too close while the catch is running
  (if (and (Utilities|IsValid OtherActor) (>= (Math|Float|Absolute(Float) (.X (Math|Vector|BreakVector (Transformation|GetVelocity)))) 1e+01))
    (bind _outhit (Collision|LineTraceByChannel _returnvalue _returnvalue_2 "TraceTypeQuery5" false 0 "None"))
    (Class|VertUtilities|VERTTakePointDamage OtherActor (Variables|Damage|GetPassive%20Damage) "/Game/Blueprints/Weapons/DamageTypes/DamageTaken/BP_DamageType_Taken_CatchPhysical.BP_DamageType_Taken_CatchPhysical_C" (Math|Vector|Normalize (- _returnvalue_2 _returnvalue)) _outhit (Variables|Damage|GetPassive%20Knockback) (Variables|Damage|GetPassive%20Knockback%20Scaling) 0.2 (Pawn|GetController) self)))

(event Custom|Notify_ChestPountAnimationEnd
  (Utilities|Time|SetTimerbyEvent (delegate Custom|RoarFinished) 1.5))

(event Custom|RoarFinished
  (Utilities|Casting|CastToBP_GorillaAnimation (Components|SkeletalMesh|GetAnimInstance (Variables|Character|GetMesh))))

(event EventExecutePunchAttack
  (|CallParentFunction))

(event EventExecuteSlamAttack
  (|CallParentFunction))

(event EventExecuteRoarAttack
  (Utilities|Casting|CastToBP_GorillaAnimation (Components|SkeletalMesh|GetAnimInstance (Variables|Character|GetMesh))))

(event Custom|Recieve%20Slam%20Stop%20Tracing
  (bind _aoechecker (Variables|Default|GetAoEChecker))
  (bind _slam_radial_config (Variables|Damage|GetSlam%20Radial%20Config))
  (bind (_infiniteammo _infiniteclip _ammoperclip _initialclips _basedamage _damagetype _timebetweenshots _firingmode _burstnumberofshots _bursttimebetweenshots _baseknockback _knockbackscaling) (Utilities|Struct|BreakWeaponData _slam_radial_config))
  (bind _returnvalue (Transformation|GetWorldLocation _aoechecker))
  (bind (_x _y _z) (Math|Vector|BreakVector _returnvalue))
  (Variables|Attacks|SetTrace%20For%20Slam%20Hits false)
  (Class|VertUtilities|VERTApplyRadialDamage self (Math|Conversions|ToFloat(Integer) _basedamage) _baseknockback _knockbackscaling 0.0 (Math|Vector|MakeVector _x _y (- _z (* (Components|Capsule|GetScaledCapsuleHalfHeight (Variables|Default|GetCapsuleComponent)) 0.75))) (Variables|Attacks|GetSlam%20Radius) "/Game/Blueprints/Weapons/DamageTypes/DamageTaken/BP_DamageType_Taken_CatchRadial.BP_DamageType_Taken_CatchRadial_C" (Utilities|Array|MakeArray 0) self (Pawn|GetController) false "ECC_Visibility"))

(event Custom|Recieve%20Punch%20Start%20Tracing
  (bind _punchhitactors (Variables|Attacks|GetPunchHitActors))
  (Variables|Attacks|SetTrace%20For%20Punch%20Hits true)
  (Utilities|Array|Clear _punchhitactors)
  (Variables|Attacks|SetFirst%20Trace true)
  (Utilities|Array|AddUnique _punchhitactors self))

(event Custom|Recieve%20Punch%20Stop%20Tracing
  (Variables|Attacks|SetTrace%20For%20Punch%20Hits false))

(event Custom|Recieve%20Slam%20Start%20Tracing
  (bind _slamhitactors (Variables|Attacks|GetSlamHitActors))
  (Variables|Attacks|SetTrace%20For%20Slam%20Hits true)
  (Utilities|Array|Clear _slamhitactors)
  (Variables|Attacks|SetFirst%20Trace true)
  (Utilities|Array|AddUnique _slamhitactors self))

(event EventTick
  (params (DeltaSeconds :type Float%20%28single-precision%29))
  (bind _returnvalue (Pawn|GetController))
  (bind _self self)
  (bind _mesh (Variables|Character|GetMesh))
  (bind _slam_weapon_config (Variables|Damage|GetSlam%20Weapon%20Config))
  (Utilities|FlowControl|Sequence
    (:then_0
      (if (Variables|Attacks|GetTrace%20For%20Slam%20Hits)
        (bind (_out_trace_position _hit_actors) (CallFunction|MeleeWeaponTrace _mesh "L_Hand_Joint" (Variables|Attacks|GetFirst%20Trace) (Variables|Default|GetSlam%20Last%20Trace%20Location%20Left) 1e+02 "TraceTypeQuery8" (Variables|Attacks|GetSlamHitActors) _slam_weapon_config _returnvalue _self "/Game/Art/Particles/P_PlayerHit_1.P_PlayerHit_1" "/Game/WwiseAudio/Weapons/Player_Punch_Impact.Player_Punch_Impact"))
        (Variables|Default|SetSlam%20Last%20Trace%20Location%20Left _out_trace_position)
        (Variables|Attacks|SetSlamHitActors _hit_actors)
        (bind (_out_trace_position_2 _hit_actors_2) (CallFunction|MeleeWeaponTrace _mesh "R_Hand_Joint" (Variables|Attacks|GetFirst%20Trace) (Variables|Default|GetSlam%20Last%20Trace%20Location%20Right) 1e+02 "TraceTypeQuery8" (Variables|Attacks|GetSlamHitActors) _slam_weapon_config _returnvalue _self "/Game/Art/Particles/P_PlayerHit_1.P_PlayerHit_1" "/Game/WwiseAudio/Weapons/Player_Punch_Impact.Player_Punch_Impact"))
        (Variables|Default|SetSlam%20Last%20Trace%20Location%20Right _out_trace_position_2)
        (Variables|Attacks|SetSlamHitActors _hit_actors_2)
        (Variables|Attacks|SetFirst%20Trace false :!label _label)))
    (:then_1
      (if (Variables|Attacks|GetTrace%20For%20Punch%20Hits)
        (bind (_out_trace_position_3 _hit_actors_3) (CallFunction|MeleeWeaponTrace (Variables|Character|GetMesh) "L_Hand_Joint" (Variables|Attacks|GetFirst%20Trace) (Variables|Default|GetPunch%20Last%20Trace%20Location) 1.5e+02 "TraceTypeQuery8" (Variables|Attacks|GetPunchHitActors) (Variables|Damage|GetPunch%20Weapon%20Config) (Pawn|GetController) self "/Game/Art/Particles/P_PlayerHit_1.P_PlayerHit_1" "/Game/WwiseAudio/Weapons/Player_Punch_Impact.Player_Punch_Impact"))
        (Variables|Default|SetPunch%20Last%20Trace%20Location _out_trace_position_3)
        (Variables|Attacks|SetPunchHitActors _hit_actors_3)
        (goto _label)))))

(fn ConstructionScript)