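; Smart nav link proxy that makes AI CatchCharacter agents jump to the link destination.
; On reaching the link, it saves the agent's max walk speed, applies an override speed and binds to the landed event to restore it.
; It then launches the agent along a suggested custom projectile arc, shaped by arc and gravity parameters, with separate horizontal and vertical velocity multipliers.
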(event Custom|OnCatchLanded_Event_0
  (Variables|/Script/Engine.CharacterMovementComponent|SetMaxWalkSpeed (Variables|/Script/Engine.Character|GetCharacterMovement (stale EventSmartLinkReached _ascatch_character)) (stale EventSmartLinkReached _output_get)))

(event EventSmartLinkReached
  (params (Agent :type Actor%20Object%20Reference) (Destination :type Vector%20%28by%20ref%29))
  (bind _xylaunchmultiplier (Variables|Default|GetXYLaunchMultiplier))
  (bind _ascatch_character (Utilities|Casting|CastToCatchCharacter Agent))
  (Utilities|FlowControl|Sequence
    (:then_0
      (bind _output_get (Variables|Default|SetSaved%20Max%20Walk%20Speed (Variables|/Script/Engine.CharacterMovementComponent|GetMaxWalkSpeed (Variables|/Script/Engine.Character|GetCharacterMovement _ascatch_character))))
      (EventDispatchers|AssignOnCatchLanded _ascatch_character (delegate Custom|OnCatchLanded_Event_0)))
    (:then_1
      (Variables|/Script/Engine.CharacterMovementComponent|SetMaxWalkSpeed (Variables|/Script/Engine.Character|GetCharacterMovement _ascatch_character) (Variables|Default|GetOverride%20Pawn%20Walk%20Speed)))
    (:then_2
      (bind _outlaunchvelocity (Game|SuggestProjectileVelocityCustomArc (Transformation|GetActorLocation Agent) Destination (Variables|Default|GetGravity%20Override) (Variables|Default|GetArc%20Param)))
      (Character|LaunchCharacter _ascatch_character (Math|Vector|MakeVector (* (.X (Math|Vector|BreakVector _outlaunchvelocity)) _xylaunchmultiplier) (* (.Y (Math|Vector|BreakVector _outlaunchvelocity)) _xylaunchmultiplier) (* (.Z (Math|Vector|BreakVector _outlaunchvelocity)) (Variables|Default|GetZLaunchMultiplier))) true true))))

(fn ConstructionScript)