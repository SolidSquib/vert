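; Trigger volume actor that gives a referenced BP_ChargerPig its checkpoints and detection state for characters inside its box.
; On BeginPlay it casts the pig reference and passes CheckpointA and CheckpointB to SetupCheckpoints.
; Box overlaps keep a list of characters other than the pig, with debug prints on enter and exit.
; Every Tick it calls the pig's VisionDetection with whether that list is non-empty.
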(event OnComponentBeginOverlap(TriggerBox)
  (params (OverlappedComponent :type Primitive%20Component%20Object%20Reference) (OtherActor :type Actor%20Object%20Reference) (OtherComp :type Primitive%20Component%20Object%20Reference) (OtherBodyIndex :type Integer) (bFromSweep :type Boolean) (SweepResult :type Hit%20Result%20Structure%20%28by%20ref%29))
  (bind _ascharacter (Utilities|Casting|CastToCharacter OtherActor))
  (Utilities|IsValid _ascharacter
    (:Is%20Valid
      (if (and (!= OtherActor (Variables|Default|GetChargerPig_Reference)) (== (Utilities|Array|FindItem (Variables|Default|GetLocalActors) OtherActor) -1))
        (Utilities|Array|AddUnique (Variables|Default|GetLocalActors) OtherActor)
        (Development|PrintString "Player Entered")))))

(event OnComponentEndOverlap(TriggerBox)
  (params (OverlappedComponent :type Primitive%20Component%20Object%20Reference) (OtherActor :type Actor%20Object%20Reference) (OtherComp :type Primitive%20Component%20Object%20Reference) (OtherBodyIndex :type Integer))
  (bind _ascharacter (Utilities|Casting|CastToCharacter OtherActor))
  (Utilities|IsValid _ascharacter
    (:Is%20Valid
      (if (!= OtherActor (Variables|Default|GetChargerPig_Reference))
        (Utilities|Array|RemoveItem (Variables|Default|GetLocalActors) _ascharacter)
        (Development|PrintString "Player Exited")))
    (:Is%20Not%20Valid
      (Development|PrintString "CAST FAILED"))))

(event EventBeginPlay
  (bind _asbp_charger_pig (Utilities|Casting|CastToBP_ChargerPig (Variables|Default|GetChargerPig_Reference))
    (:then
      (bind _output_get (Variables|Default|SetBP_ChargerPig_Reference _asbp_charger_pig))
      (Default|SetupCheckpoints _output_get (Variables|Default|GetCheckpointA) (Variables|Default|GetCheckpointB)))
    (:CastFailed
      (Development|PrintString "ChargerPig Reference Missing"))))

(event EventTick
  (params (DeltaSeconds :type Float%20%28single-precision%29))
  (bind _bp_chargerpig_reference (Variables|Default|GetBP_ChargerPig_Reference))
  (Utilities|IsValid _bp_chargerpig_reference
    (:Is%20Valid
      (Default|VisionDetection _bp_chargerpig_reference (> (Utilities|Array|Length (Variables|Default|GetLocalActors)) 0)))))

(fn ConstructionScript)