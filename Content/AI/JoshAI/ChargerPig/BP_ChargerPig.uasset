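; AI charger pig enemy that charges between two checkpoints while targets are detected and dies when its health runs out.
; Tick drives the Blackboard state and target location, flipping checkpoints on arrival and returning to Idle once no targets remain.
; VisionDetection sets the detection flag, and SetupCheckpoints supplies the endpoints and trigger radius.
; While charging, two helmet boxes deal knockback damage to Characters, tracking overlaps to prevent repeat hits.
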(event OnComponentBeginOverlap(Box_Helmet2)
  (params (OverlappedComponent :type Primitive%20Component%20Object%20Reference) (OtherActor :type Actor%20Object%20Reference) (OtherComp :type Primitive%20Component%20Object%20Reference) (OtherBodyIndex :type Integer) (bFromSweep :type Boolean) (SweepResult :type Hit%20Result%20Structure%20%28by%20ref%29))
  ;[1 1 1] If player touches the Helmet Collision they take damage
  (Development|PrintString "Helmet2 Overlap")
  (CallFunction|OnTargetOverlap OtherActor SweepResult))

(event OnComponentEndOverlap(Box_Helmet2)
  (params (OverlappedComponent :type Primitive%20Component%20Object%20Reference) (OtherActor :type Actor%20Object%20Reference) (OtherComp :type Primitive%20Component%20Object%20Reference) (OtherBodyIndex :type Integer))
  ;[1 1 1] When player leaves the collision - remove from array
  (CallFunction|OnTargetExit OtherActor))

(event OnComponentBeginOverlap(Box_Helmet1)
  (params (OverlappedComponent :type Primitive%20Component%20Object%20Reference) (OtherActor :type Actor%20Object%20Reference) (OtherComp :type Primitive%20Component%20Object%20Reference) (OtherBodyIndex :type Integer) (bFromSweep :type Boolean) (SweepResult :type Hit%20Result%20Structure%20%28by%20ref%29))
  ;[1 1 1] If player touches the Helmet Collision they take damage
  (Development|PrintString "Helmet1 Overlap")
  (CallFunction|OnTargetOverlap OtherActor SweepResult))

(event OnComponentBeginOverlap(Capsule_Behind)
  (params (OverlappedComponent :type Primitive%20Component%20Object%20Reference) (OtherActor :type Actor%20Object%20Reference) (OtherComp :type Primitive%20Component%20Object%20Reference) (OtherBodyIndex :type Integer) (bFromSweep :type Boolean) (SweepResult :type Hit%20Result%20Structure%20%28by%20ref%29)))

(event OnComponentEndOverlap(Box_Helmet1)
  (params (OverlappedComponent :type Primitive%20Component%20Object%20Reference) (OtherActor :type Actor%20Object%20Reference) (OtherComp :type Primitive%20Component%20Object%20Reference) (OtherBodyIndex :type Integer))
  ;[1 1 1] When player leaves the collision - remove from array
  (CallFunction|OnTargetExit OtherActor))

(event Custom|Cry%20Delay%20Timer%20Done
  (Utilities|FlowControl|DoOnce false) ; enters at Reset
)

(event EventTakeDamageFailed)

(event EventBeginPlay
  (bind _self self)
  (bind _returnvalue (AI|GetAIController _self))
  (bind _returnvalue_2 (AI|GetBlackboard _returnvalue))
  ;[1 1 1] Assign Startup References
  (Utilities|IsValid _returnvalue_2
    (:Is%20Valid
      (Variables|Default|SetBlackboard_Reference _returnvalue_2)
      (bind _asbp_charger_pig_animation (Utilities|Casting|CastToBP_ChargerPigAnimation (Components|SkeletalMesh|GetAnimInstance (Variables|Character|GetMesh))))
      (Variables|Default|SetBP_AnimInstance _asbp_charger_pig_animation))
    (:Is%20Not%20Valid
      (Development|PrintString "ChargerPig BeginPlay - Blackboard IsNotValid"))))

(event EventTakeDamageSucceeded
  (params (actualDamageTaken :type Float%20%28single-precision%29))
  (bind _output_get (Variables|Default|SetHealth (- (Variables|Default|GetHealth) actualDamageTaken)))
  (if (<= _output_get 0.0)
    (bind _returnvalue (Effects|SpawnEmitteratLocation "/Game/Art/Particles/P_PlayerDeath.P_PlayerDeath" (Transformation|GetActorLocation)))
    (Effects|Components|ParticleSystem|SetColorParameter _returnvalue "PlayerDeath_Col" "(R=0.012801,G=0.002870,B=0.065000,A=1.000000)")
    (Class|VertCharacterBase|Die)))

(event EventTick
  (params (DeltaSeconds :type Float%20%28single-precision%29))
  (Utilities|SetBlackboardReferenceLocal
    (:Valid
      (if (Utilities|Enum|Equal(Enum) (Utilities|Enum|ByteToEnumEnum_ChargerPig (Class|BlackboardComponent|GetValueasEnum (Variables|Default|GetBlackboard_Reference) (Variables|BlackboardReferences|GetBB_CurrentState))) "NewEnumerator2") ; Are we currently charging
        (if (<= (Math|Vector|VectorLength (- (Transformation|GetActorLocation) (.NextCheckpointLocation (CallFunction|GetCheckpoint)))) (Variables|Default|GetCheckpointTriggerDistance)) ; Are we in range of target Checkpoint?
          ;[1 1 1] Switch to next Checkpoint
          (if (Variables|Checkpoints|GetTargetCheckpointIsA)
            (Variables|Checkpoints|SetTargetCheckpointIsA false)
            (else
              (Variables|Checkpoints|SetTargetCheckpointIsA true)))
          ;[1 1 1] Update Blackboard value
          (AI|Components|Blackboard|SetValueasVector (Variables|Default|GetBlackboard_Reference) (Variables|BlackboardReferences|GetBB_TargetLocation) (.NextCheckpointLocation (CallFunction|GetCheckpoint)))
          (Animation|StopAnimMontage "/Game/Art/Characters/ChargerPig/Animations/Anim_ChargerPig_Skid.Anim_ChargerPig_Skid")
          (if (not (Variables|Checkpoints|GetTargetsDetected))
            ;[1 1 1] Set State to Idle if no targets detected
            (AI|Components|Blackboard|SetValueasEnum (Variables|Default|GetBlackboard_Reference) (Variables|BlackboardReferences|GetBB_CurrentState) (Utilities|Enum|LiteralenumEnum_ChargerPig "NewEnumerator0"))
            (Development|PrintString "CurrentState: Idle Set")
            (Utilities|FlowControl|DoOnce false
              (:Completed
                (Class|AkGameplayStatics|PostEvent "/Game/WwiseAudio/Piggy/Rhino_Cry.Rhino_Cry" self false)
                (Utilities|Time|SetTimerbyEvent (delegate Custom|Cry%20Delay%20Timer%20Done) 5.0)))))
        (elif (Variables|Checkpoints|GetTargetsDetected) ; Should we be in combat?
          ;[1 1 1] Setting State to Combat if enemies detected
          (AI|Components|Blackboard|SetValueasEnum (Variables|Default|GetBlackboard_Reference) (Variables|BlackboardReferences|GetBB_CurrentState) (Utilities|Enum|LiteralenumEnum_ChargerPig "NewEnumerator2"))
          (Development|PrintString "CurrentState: Combat Set"))))))

(fn ConstructionScript)

(fn VisionDetectionTrace
  (bind _mesh (Variables|Character|GetMesh))
  (bind _returnvalue (Transformation|GetWorldLocation _mesh))
  (bind (_outhit _returnvalue_2) (Collision|BoxTraceByChannel (+ _returnvalue "0, 0,160.000000") (+ _returnvalue "100.000000, 0,160.000000") (Math|Vector|MakeVector 1e+02 1e+02 (Components|Capsule|GetScaledCapsuleHalfHeight (Variables|Default|GetCapsuleComponent))) "0, 0, 0" "TraceTypeQuery1" false (Utilities|Array|MakeArray (Components|GetOwner)) "ForDuration"))
  (if _returnvalue_2
    (Utilities|Casting|CastToCharacter (.HitActor (Collision|BreakHitResult _outhit))
      (:then
        (LocalVariables|SetWasTargetDetected true))
      (:CastFailed
        (LocalVariables|SetWasTargetDetected false :!label _label)))
    (else
      (goto _label))))

(fn GetCheckpoint
  (bind _checkpointa (Variables|Default|GetCheckpointA))
  (bind _checkpointb (Variables|Default|GetCheckpointB))
  (bind _targetcheckpointisa (Variables|Checkpoints|GetTargetCheckpointIsA))
  (bind _returnvalue (select _targetcheckpointisa _checkpointa _checkpointb))
  (return _returnvalue (Transformation|GetWorldLocation _returnvalue)))

(fn VisionDetection
  (params (Detected? :type Boolean))
  (Variables|Checkpoints|SetTargetsDetected Detected?))

(fn SetupCheckpoints
  (params (CheckpointA :type Sphere%20Component%20Object%20Reference) (CheckpointB :type Sphere%20Component%20Object%20Reference))
  (bind (_nextcheckpoint _nextcheckpointlocation) (CallFunction|GetCheckpoint))
  (Utilities|IsValid CheckpointA
    (:Is%20Valid
      (Variables|Default|SetCheckpointA CheckpointA)
      (Utilities|IsValid CheckpointB
        (:Is%20Valid
          (Variables|Default|SetCheckpointB CheckpointB)
          (Variables|Default|SetCheckpointTriggerDistance (Components|Sphere|GetScaledSphereRadius CheckpointB))
          (Development|PrintString "Checkpoints Set" false false)
          ;[1 1 1] Setting initial starting position
          (if (Variables|Checkpoints|GetStartCheckpointA)
            (Variables|Checkpoints|SetTargetCheckpointIsA false)
            (else
              (Variables|Checkpoints|SetTargetCheckpointIsA true)))
          (AI|Components|Blackboard|SetValueasVector (Variables|Default|GetBlackboard_Reference) (Variables|BlackboardReferences|GetBB_TargetLocation) _nextcheckpointlocation)
          (Development|PrintString "Starting Checkpoint is set")
          (Development|PrintString (Utilities|GetDisplayName _nextcheckpoint)))
        (:Is%20Not%20Valid
          (Development|PrintString "ChargerPig_SetupCheckpoints - Checkpont B Is Not Valid"))))
    (:Is%20Not%20Valid
      (Development|PrintString "ChargerPig_SetupCheckpoints - Checkpont A Is Not Valid"))))

(fn OnTargetOverlap
  (params (Other%20Actor :type Actor%20Object%20Reference) (Hit%20Results :type Hit%20Result%20Structure))
  (Utilities|SetBlackboardReferenceLocal
    (:Valid
      (if (Utilities|Enum|Equal(Enum) (Utilities|Enum|ByteToEnumEnum_ChargerPig (Class|BlackboardComponent|GetValueasEnum (Variables|Default|GetBlackboard_Reference) (Variables|BlackboardReferences|GetBB_CurrentState))) "NewEnumerator2")
        (bind _ascharacter (Utilities|Casting|CastToCharacter Other%20Actor))
        (Utilities|IsValid _ascharacter
          (:Is%20Valid
            (if (== (Utilities|Array|FindItem (Variables|Default|GetOverlappingActors_Horn) _ascharacter) -1)
              (Class|VertUtilities|VERTTakePointDamage _ascharacter (Variables|Default|GetDamage) "/Game/Blueprints/Weapons/DamageTypes/DamageTaken/BP_DamageType_Taken_ForgeHammer.BP_DamageType_Taken_ForgeHammer_C" (Math|Vector|Normalize (Math|Vector|MakeVector (.X (Math|Vector|BreakVector (- (Transformation|GetActorLocation _ascharacter) (Transformation|GetActorLocation)))) (.Y (Math|Vector|BreakVector (- (Transformation|GetActorLocation _ascharacter) (Transformation|GetActorLocation)))) 0.0)) Hit%20Results (Variables|Default|GetKnockback) 0.0 0.0 (Pawn|GetController) self)
              (Utilities|Array|AddUnique (Variables|Default|GetOverlappingActors_Horn) _ascharacter)
              (Effects|SpawnEmitterAttached "/Game/Art/Particles/P_DropPod_Impact.P_DropPod_Impact" (Variables|Character|GetMesh) "FX_Socket_Helmet" "0, 0, 0" "0, 0, 0" "SnapToTargetIncludingScale"))))))))

(fn OnTargetExit
  (params (OtherActor :type Actor%20Object%20Reference))
  (bind _ascharacter (Utilities|Casting|CastToCharacter OtherActor))
  (Utilities|IsValid _ascharacter
    (:Is%20Valid
      (if (not (== (Utilities|Array|FindItem (Variables|Default|GetOverlappingActors_Horn) _ascharacter) -1))
        (Utilities|Array|RemoveItem (Variables|Default|GetOverlappingActors_Horn) _ascharacter)))))