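; Gorilla AI character with punch, slam and roar attacks, whose startup and section start are delegated to BP_Gorilla_AIController.
; Punches sweep box traces between successive left-hand socket positions on Tick, flattened to Y=0, hitting each character once per swing.
; Slam damages characters tracked by a trigger box, while roar applies radial damage from the mouth socket.
; It also ignores PlayerPod damage and drives an enrage glow through a material timeline.
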(event OnComponentBeginOverlap(Box_SlamTrigger)
  (params (OverlappedComponent :type Primitive%20Component%20Object%20Reference) (OtherActor :type Actor%20Object%20Reference) (OtherComp :type Primitive%20Component%20Object%20Reference) (OtherBodyIndex :type Integer) (bFromSweep :type Boolean) (SweepResult :type Hit%20Result%20Structure%20%28by%20ref%29))
  ;[1 1 1] SlamTrigger - adds targets to array
  (bind _ascharacter (Utilities|Casting|CastToCharacter OtherActor))
  (if (and (!= _ascharacter self) (== (Utilities|Array|FindItem (Variables|Slam|GetOverlappingActors_SlamTrigger) _ascharacter) -1))
    (Utilities|Array|AddUnique (Variables|Slam|GetOverlappingActors_SlamTrigger) _ascharacter)))

(event OnComponentBeginOverlap(Box_PunchTrigger)
  (params (OverlappedComponent :type Primitive%20Component%20Object%20Reference) (OtherActor :type Actor%20Object%20Reference) (OtherComp :type Primitive%20Component%20Object%20Reference) (OtherBodyIndex :type Integer) (bFromSweep :type Boolean) (SweepResult :type Hit%20Result%20Structure%20%28by%20ref%29))
  ;[1 1 1] PunchTrigger - adds targets to array
  (bind _ascharacter (Utilities|Casting|CastToCharacter OtherActor))
  (if (and (!= _ascharacter self) (== (Utilities|Array|FindItem (Variables|Punch|GetOverlappingActors_PunchTrigger) _ascharacter) -1))
    (Utilities|Array|AddUnique (Variables|Punch|GetOverlappingActors_PunchTrigger) _ascharacter)))

(event OnComponentEndOverlap(Box_PunchTrigger)
  (params (OverlappedComponent :type Primitive%20Component%20Object%20Reference) (OtherActor :type Actor%20Object%20Reference) (OtherComp :type Primitive%20Component%20Object%20Reference) (OtherBodyIndex :type Integer))
  ;[1 1 1] PunchTrigger - adds targets to array
  (bind _ascharacter (Utilities|Casting|CastToCharacter OtherActor))
  (Utilities|Array|RemoveItem (Variables|Punch|GetOverlappingActors_PunchTrigger) _ascharacter))

(event OnComponentEndOverlap(Box_SlamTrigger)
  (params (OverlappedComponent :type Primitive%20Component%20Object%20Reference) (OtherActor :type Actor%20Object%20Reference) (OtherComp :type Primitive%20Component%20Object%20Reference) (OtherBodyIndex :type Integer))
  ;[1 1 1] SlamTrigger - adds targets to array
  (bind _ascharacter (Utilities|Casting|CastToCharacter OtherActor))
  (Utilities|Array|RemoveItem (Variables|Slam|GetOverlappingActors_SlamTrigger) _ascharacter))

(event Custom|SetEnragingValues
  (bind _mesh (Variables|Character|GetMesh))
  ;[1 1 1] Change Gorilla Glow to Red during Enrage
  (Utilities|FlowControl|DoOnce false
    (:Completed
      (Components|Timeline|SetPlayRate (Variables|Default|GetEnrageMaterialColours) 1.0) ; Default is 1 second
      (bind (_direction _glow_pow _glow_col) (Timeline|EnrageMaterialColours PlayFromStart)
        (:Update
          (Rendering|Material|SetScalarParameterValueonMaterials _mesh "Glow_Col" _glow_col)
          (Rendering|Material|SetScalarParameterValueonMaterials _mesh "Glow_Pow" _glow_pow))))))

(event Custom|Stop%20Punch%20Hit%20Tracing
  ;[1 1 1] Punch/Swipe Hit Tracing
  (Variables|Punch|SetStartPunchTracing false)
  (Utilities|Array|Clear (Variables|Punch|GetPunch_HitTrace_Actors)))

(event Custom|StartRoarDamage
  (bind _self self)
  ;[1 1 1] Roar
  (if (Variables|Roar|GetRoarTestToggle)
    (Variables|Roar|SetRoarTestToggle false)
    (Class|VertUtilities|VERTApplyRadialDamage _self (Math|Conversions|ToFloat(Integer) (Variables|Roar|GetRoarDamage)) (Variables|Roar|GetRoarKnockback) 1.0 0.1 (Transformation|GetSocketLocation (Variables|Character|GetMesh) "Socket_Mouth") (Variables|Roar|GetRoarRadius) "/Game/Blueprints/Weapons/DamageTypes/DamageTaken/BP_DamageType_Taken_Punch.BP_DamageType_Taken_Punch_C" (Utilities|Array|MakeArray (Components|GetOwner)) _self (Pawn|GetController (Variables|Default|GetInstigator)) false "ECC_Visibility")))

(event Custom|ApplyRoarDamage
  ;[1 1 1] Roar OLD - Damage Called from GorillaAnimBP using Notifies on Attack_Roar Montage
)

(event Custom|Start%20Punch%20Hit%20Tracing
  ;[1 1 1] Punch/Swipe Hit Tracing
  (Variables|Punch|SetStartPunchTracing true))

(event Custom|StartGorillaAI
  ;[1 1 1] Start Gorilla AI - called by GorillaStartTrigger
  (Development|PrintString "StartGorillaAI Event Called")
  (bind _asbp_gorilla_aicontroller (Utilities|Casting|CastToBP_Gorilla_AIController (Pawn|GetController))
    (:then
      (Development|PrintString "AIController Cast Success")
      (Default|StartSection _asbp_gorilla_aicontroller))
    (:CastFailed
      (Development|PrintString "AIController Cast Failed"))))

(event Custom|Apply%20Slam%20Damage
  (bind _self self)
  (bind _self_2 self)
  (bind _returnvalue (Transformation|GetActorLocation _self_2))
  (bind _returnvalue_2 (Transformation|GetActorLocation _self))
  (bind (_x _y _z) (Math|Vector|BreakVector _returnvalue))
  (bind (_x_2 _y_2 _z_2) (Math|Vector|BreakVector _returnvalue_2))
  ;[1 1 1] Slam Damage
  (Effects|SpawnEmitteratLocation "/Game/Art/Particles/P_Monkey_Impact.P_Monkey_Impact" (Math|Vector|MakeVector (+ _x_2 3e+02) _y_2 (- _z_2 (Components|Capsule|GetScaledCapsuleHalfHeight (Variables|Default|GetCapsuleComponent)))))
  (bind _array_element (Utilities|Array|ForEachLoopwithBreak (Variables|Slam|GetOverlappingActors_SlamTrigger))
    (:LoopBody
      (bind _ascharacter (Utilities|Casting|CastToCharacter _array_element))
      (Utilities|IsValid _ascharacter
        (:Is%20Valid
          (Class|VertUtilities|VERTTakePointDamage _ascharacter (Math|Conversions|ToFloat(Integer) (Variables|Slam|GetSlamDamage)) "/Game/Blueprints/Weapons/DamageTypes/DamageTaken/BP_DamageType_Taken_ForgeHammer.BP_DamageType_Taken_ForgeHammer_C" (Math|Vector|MakeVector 0.0 0.0 1.0) (Collision|MakeHitResult false false 0.0 (Math|Vector|MakeVector (.X (Math|Vector|BreakVector (Transformation|GetActorLocation _ascharacter))) (.Y (Math|Vector|BreakVector (Transformation|GetActorLocation _ascharacter))) (- (.Z (Math|Vector|BreakVector (Transformation|GetActorLocation _ascharacter))) (Components|Capsule|GetScaledCapsuleHalfHeight (Variables|/Script/Engine.Character|GetCapsuleComponent _ascharacter)))) (Math|Vector|MakeVector _x _y (- _z (Components|Capsule|GetScaledCapsuleHalfHeight (Variables|Default|GetCapsuleComponent)))) "0, 0,-1.000000" "0.000000,0.000000,-1.000000" 0 _ascharacter 0) (Variables|Slam|GetSlamKnockback) 1.0 0.5 (Pawn|GetController (Variables|Default|GetInstigator)) self))))))

(event EventTick
  (params (DeltaSeconds :type Float%20%28single-precision%29))
  ;[1 1 1] Punch/Swipe Hit Tracing
  (if (Variables|Punch|GetStartPunchTracing)
    (CallFunction|PunchHitTrace)
    (Utilities|FlowControl|DoOnce false :!label _label
      (:Completed
        (Utilities|FlowControl|Delay 0.5) ; makes sure punch hit tracing stops
        (Variables|Punch|SetStartPunchTracing false)))
    (else
      (goto _label Reset))))

(event Game|Damage|EventAnyDamage
  (params (Damage :type Float%20%28single-precision%29) (DamageType :type Damage%20Type%20Object%20Reference) (InstigatedBy :type Controller%20Object%20Reference) (DamageCauser :type Actor%20Object%20Reference))
  ;[1 0 0] NEEDS CHECKING
  (if (!= DamageType "/Game/Blueprints/Weapons/DamageTypes/DamageTaken/BP_DamageType_Taken_PlayerPod.BP_DamageType_Taken_PlayerPod")
    (|CallParentFunction Damage DamageType InstigatedBy DamageCauser)))

(event EventBeginPlay
  (bind _asbp_gorilla_aicontroller (Utilities|Casting|CastToBP_Gorilla_AIController (Pawn|GetController)))
  (Default|StartupGorillaSequence _asbp_gorilla_aicontroller))

(event EventOnLanded
  (params (Hit :type Hit%20Result%20Structure%20%28by%20ref%29))
  (Class|AkGameplayStatics|PostEvent "/Game/WwiseAudio/Catch/Gorilla_Land.Gorilla_Land" self false))

(fn ConstructionScript)

(fn PunchHitTrace
  (bind _mesh (Variables|Character|GetMesh))
  (bind _returnvalue (Transformation|GetSocketLocation _mesh "Socket_LeftHand"))
  (if (Variables|Punch|GetSetStartingTracePosition)
    (Variables|Punch|SetPunch_HitTrace_LastPosition _returnvalue)
    (Variables|Punch|SetSetStartingTracePosition false)
    (else
      (Variables|Punch|SetPunch_HitTrace_LastPosition (Variables|Punch|GetPunch_HitTrace_NewPosition))))
  (Variables|Punch|SetPunch_HitTrace_NewPosition _returnvalue)
  (Variables|Punch|SetPunch_HtTrace_Rotation (Transformation|GetSocketRotation _mesh "Socket_LeftHand"))
  (bind _outhits (Class|KismetSystemLibrary|BoxTraceMulti (Math|Vector|MakeVector (.X (Math|Vector|BreakVector (Variables|Punch|GetPunch_HitTrace_LastPosition))) 0.0 (.Z (Math|Vector|BreakVector (Variables|Punch|GetPunch_HitTrace_LastPosition)))) (Math|Vector|MakeVector (.X (Math|Vector|BreakVector (Variables|Punch|GetPunch_HitTrace_NewPosition))) 0.0 (.Z (Math|Vector|BreakVector (Variables|Punch|GetPunch_HitTrace_NewPosition)))) "40.000000,300.000000,60.000000" "0, 0, 0" "TraceTypeQuery8" false 0 "ForOneFrame" true))
  (bind _array_element (Utilities|Array|ForEachLoopwithBreak _outhits)
    (:LoopBody
      (Utilities|Casting|CastToCharacter (.HitActor (Collision|BreakHitResult _array_element)))
      (if (== (Utilities|Array|FindItem (Variables|Punch|GetPunch_HitTrace_Actors) (.HitActor (Collision|BreakHitResult _array_element))) -1)
        (Utilities|Array|AddUnique (Variables|Punch|GetPunch_HitTrace_Actors) (.HitActor (Collision|BreakHitResult _array_element)))
        (Class|VertUtilities|VERTTakePointDamage (.HitActor (Collision|BreakHitResult _array_element)) (Variables|Punch|GetPunchDamage) "/Game/Blueprints/Weapons/DamageTypes/DamageTaken/BP_DamageType_Taken_ForgeHammer.BP_DamageType_Taken_ForgeHammer_C" (Math|Vector|Normalize (Math|Vector|MakeVector (.X (Math|Vector|BreakVector (- (Transformation|GetActorLocation (.HitActor (Collision|BreakHitResult _array_element))) (Transformation|GetActorLocation)))) 0.0 (.Z (Math|Vector|BreakVector (- (Transformation|GetActorLocation (.HitActor (Collision|BreakHitResult _array_element))) (Transformation|GetActorLocation)))))) _array_element (Variables|Punch|GetPunchKnockback) 1.0 0.2 (Pawn|GetController) self)))))