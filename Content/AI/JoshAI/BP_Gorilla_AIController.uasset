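; AI controller for the Gorilla in a timed arena section, running its behavior tree and writing states to the blackboard.
; Tick triggers slam and punch attacks from trigger overlaps and cooldowns, while timers request target switches and the arena exit.
; ChangeState can save the current state for resuming and cancel the active MoveTo for instant interrupts.
; Enrage, roar and all-players-dead idle logic are present but disconnected.
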(event Custom|ManualEnrage
  ;[1 1 1] Setting Enrage based on time instead of health due to short fight duration
  (AI|Components|Blackboard|SetValueasBool (Variables|Default|GetBlackboardReference) (Variables|BlackboardReferences|GetIsEnraged) true)
  (CallFunction|ChangeState "NewEnumerator6" true true))

(event Custom|KillGorillaEvent
  ;[1 1 1] Kills the Gorilla after x seconds
  (Variables|Default|SetSwitchToExit true))

(event Custom|StartSection
  ;[1 1 1] START GORILLA GAMEPLAY - called when Players enter Arena Trigger
  (Development|PrintString "GORILLA SECTION")
  (CallFunction|ChangeState "NewEnumerator3" false false))

(event Custom|TriggeredEvent
  ;[1 1 1] Creating a looping event to change targeted player
  (Variables|Default|SetChooseNewTarget true))

(event Custom|SlamCooldownComplete
  ;[1 1 1] Slam
  (Variables|Attacking|Slam|SetSlamReady true))

(event Custom|RoarCooldownComplete
  ;[1 1 1] Roar OLD
  (Variables|Attacking|Roar|SetRoarReady true))

(event Custom|PunchCooldownComplete
  ;[1 1 1] Punch
  (Variables|Attacking|Punch|SetPunchReady true))

(event Custom|StartGorillaActive
  ;[1 1 1] Called when the Gorilla reaches its starting checkpoint
  ;[1 1 1] Creating a looping event to change targeted player
  (Utilities|Time|SetTimerbyEvent (delegate Custom|TriggeredEvent) (Variables|Default|GetSwitchPlayerTimer) true)
  ;[1 1 1] Kills the Gorilla after x seconds
  (Utilities|Time|SetTimerbyEvent (delegate Custom|KillGorillaEvent) 6e+01))

(event Custom|StartAttackGlobalCooldown
  ;[1 1 1] Global cooldown between attacks
  (Development|PrintString "AttackGlobalCooldown Started")
  (Variables|Attacking|SetAttackReady false)
  (Utilities|Time|SetTimerbyEvent (delegate Custom|AttackGlobalCooldownComplete) (Variables|Attacking|GetAttackGlobalCooldown)))

(event Custom|AttackGlobalCooldownComplete
  ;[1 1 1] Global cooldown between attacks
  (Variables|Attacking|SetAttackReady true)
  (Development|PrintString "AttackCooldownComplete"))

(event EventTick
  (params (DeltaSeconds :type Float%20%28single-precision%29))
  (bind _blackboardreference (Variables|Default|GetBlackboardReference))
  (bind _currentstate (Variables|BlackboardReferences|GetCurrentState))
  (bind _returnvalue (Class|BlackboardComponent|GetValueasEnum _blackboardreference _currentstate))
  (Utilities|IsValid (Variables|Default|GetBlackboardReference)
    (:Is%20Valid
      (Utilities|IsValid (Variables|References|GetBP_GorillaReference)
        (:Is%20Valid
          (Utilities|FlowControl|Sequence
            (:then_0
              ;[1 1 1] Slam
              (bind _slammed (CallFunction|Slam))
              (if _slammed
                (CallFunction|ChangeState "NewEnumerator7" true true)
                (Utilities|Time|SetTimerbyEvent (delegate Custom|SlamCooldownComplete) (Variables|Attacking|Slam|GetSlamCooldown))
                (CallFunction|StartAttackGlobalCooldown)))
            (:then_1
              ;[1 1 1] Punch
              (if (Math|Boolean|ANDBoolean (> (Utilities|Array|Length (Variables|/Game/AI/JoshAI/BP_Gorilla.BP_Gorilla_C|GetOverlappingActors_PunchTrigger (Variables|References|GetBP_GorillaReference))) 0) (Variables|Attacking|Punch|GetPunchReady) (Variables|Attacking|GetAttackReady) (Math|Boolean|ORBoolean (== _returnvalue (Utilities|Enum|LiteralenumEnum_Gorilla_AIState "NewEnumerator2")) (== _returnvalue (Utilities|Enum|LiteralenumEnum_Gorilla_AIState "NewEnumerator3")) (== _returnvalue (Utilities|Enum|LiteralenumEnum_Gorilla_AIState "NewEnumerator8"))))
                (Variables|Attacking|Punch|SetPunchReady false)
                (Animation|Montage|PlayMontage (Variables|/Script/Engine.Character|GetMesh (Variables|References|GetBP_GorillaReference)) "/Game/Art/Characters/Catch/Gorilla/Animations/Attacks/Anim_Gorilla_Attack_Punch.Anim_Gorilla_Attack_Punch" 1.0 0.0 "Punch"
                  (:then
                    (Utilities|Time|SetTimerbyEvent (delegate Custom|PunchCooldownComplete) (Variables|Attacking|Punch|GetPunchCooldown)))
                  (:OnInterrupted
                    (Development|PrintString "PUNCH INTERRUPTED")
                    (Default|StopPunchHitTracing (Variables|References|GetBP_GorillaReference))))))
            (:then_2
              ;[1 1 1] Override to Chooseplayer if player is chasing
              (if (Variables|Default|GetChooseNewTarget)
                (switch Utilities|FlowControl|Switch|SwitchonEnum_Gorilla_AIState (Utilities|Enum|ByteToEnumEnum_Gorilla_AIState (Class|BlackboardComponent|GetValueasEnum (Variables|Default|GetBlackboardReference) (Variables|BlackboardReferences|GetCurrentState)))
                  (:NewEnumerator2
                    (bind _asbp_gorilla (Utilities|Casting|CastToBP_Gorilla (Pawn|GetControlledPawn (AI|GetAIController self))))
                    (if (and (Class|VertCharacterBase|IsGrounded _asbp_gorilla) (!= (CallFunction|HowManyPlayersAreAlive) 1))
                      (Variables|Default|SetChooseNewTarget false)
                      (CallFunction|ChangeState "NewEnumerator9" true false)))
                  (:NewEnumerator9
                    (Variables|Default|SetChooseNewTarget false)))))
            (:then_3
              ;[1 1 1] Starts Exit State
              (if (Variables|Default|GetSwitchToExit)
                (switch Utilities|FlowControl|Switch|SwitchonEnum_Gorilla_AIState (Utilities|Enum|ByteToEnumEnum_Gorilla_AIState (Class|BlackboardComponent|GetValueasEnum (Variables|Default|GetBlackboardReference) (Variables|BlackboardReferences|GetCurrentState)))
                  (:NewEnumerator2
                    _)
                  (:NewEnumerator9
                    _))
                (bind _asbp_gorilla_2 (Utilities|Casting|CastToBP_Gorilla (Pawn|GetControlledPawn (AI|GetAIController self))))
                (if (Class|VertCharacterBase|IsGrounded _asbp_gorilla_2)
                  (Variables|Default|SetSwitchToExit false)
                  (CallFunction|ChangeState "NewEnumerator8" true false))))
            (:then_4)))))))

(fn ConstructionScript)

(fn Enrage
  (bind _blackboardreference (Variables|Default|GetBlackboardReference))
  (bind _currentstate (Variables|BlackboardReferences|GetCurrentState))
  (bind _returnvalue (Class|BlackboardComponent|GetValueasEnum _blackboardreference _currentstate))
  (if (not (ScalableFloat|GetValueasBool (Variables|Default|GetBlackboardReference) (Variables|BlackboardReferences|GetIsEnraged)))
    (if (and (>= (Class|HealthComponent|GetCurrentDamageModifier (Variables|/Script/Vert.VertCharacterBase|GetHealthComponent (Variables|References|GetBP_GorillaReference))) (Variables|Attacking|Enrage|GetEnrageTriggerValue)) (or (== _returnvalue (Utilities|Enum|LiteralenumEnum_Gorilla_AIState "NewEnumerator2")) (== _returnvalue (Utilities|Enum|LiteralenumEnum_Gorilla_AIState "NewEnumerator9"))))
      (AI|Components|Blackboard|SetValueasBool (Variables|Default|GetBlackboardReference) (Variables|BlackboardReferences|GetIsEnraged) true)
      (return true)
      (else
        _)))
  (return false))

(fn Slam
  (if (Math|Boolean|ANDBoolean (>= (Utilities|Array|Length (Variables|/Game/AI/JoshAI/BP_Gorilla.BP_Gorilla_C|GetOverlappingActors_SlamTrigger (Variables|References|GetBP_GorillaReference))) (Variables|Attacking|Slam|GetSlamTriggerAmount)) (Variables|Attacking|Slam|GetSlamReady) (Variables|Attacking|GetAttackReady) (== (Class|BlackboardComponent|GetValueasEnum (Variables|Default|GetBlackboardReference) (Variables|BlackboardReferences|GetCurrentState)) (Utilities|Enum|LiteralenumEnum_Gorilla_AIState "NewEnumerator2")))
    (Development|PrintString "Starting Slam")
    (Variables|Attacking|Slam|SetSlamReady false)
    (return true)
    (else
      (return false))))

(fn Roar
  (bind _blackboardreference (Variables|Default|GetBlackboardReference))
  (bind _currentstate (Variables|BlackboardReferences|GetCurrentState))
  (bind _returnvalue (Class|BlackboardComponent|GetValueasEnum _blackboardreference _currentstate))
  (if (Math|Boolean|ANDBoolean (< (Variables|Attacking|Roar|GetRoarCounter) (- (Utilities|Array|Length (Variables|Attacking|Roar|GetRoarTriggerValues)) 1)) (Variables|Attacking|Roar|GetRoarReady) (>= (Class|HealthComponent|GetCurrentDamageModifier (Variables|/Script/Vert.VertCharacterBase|GetHealthComponent (Variables|References|GetBP_GorillaReference))) (Utilities|Array|Get(acopy) (Variables|Attacking|Roar|GetRoarTriggerValues) (Variables|Attacking|Roar|GetRoarCounter))))
    (if (Math|Boolean|ANDBoolean (!= _returnvalue (Utilities|Enum|LiteralenumEnum_Gorilla_AIState "NewEnumerator0")) (!= _returnvalue (Utilities|Enum|LiteralenumEnum_Gorilla_AIState "NewEnumerator0")) (!= _returnvalue (Utilities|Enum|LiteralenumEnum_Gorilla_AIState "NewEnumerator5")) (!= _returnvalue (Utilities|Enum|LiteralenumEnum_Gorilla_AIState "NewEnumerator6")) (!= _returnvalue (Utilities|Enum|LiteralenumEnum_Gorilla_AIState "NewEnumerator7")))
      (Variables|Attacking|Roar|SetRoarReady false)
      (return true)
      (else
        (return false)))
    (else
      (return false))))

(fn CancelMoveto
  (bind _blackboardreference (Variables|Default|GetBlackboardReference))
  (bind _movetotask (Variables|BlackboardReferences|GetMoveToTask))
  (bind _returnvalue (AI|Components|Blackboard|GetValueasObject _blackboardreference _movetotask))
  (Utilities|IsValid _returnvalue
    (:Is%20Valid
      (bind _asaitask_move_to (Utilities|Casting|CastToAITask_MoveTo _returnvalue))
      (GameplayTasks|EndTask _asaitask_move_to))))

(fn ChangeState
  (params (NewState :type Enum_Gorilla_AIState%20Enum) (Override :type Boolean) (ResumePreviousState :type Boolean))
  (LocalVariables|SetLocalNewState NewState)
  (LocalVariables|SetLocalOverride Override)
  (LocalVariables|SetLocalResumePreviousState ResumePreviousState)
  (if (LocalVariables|GetLocalResumePreviousState)
    ;[1 1 1] Save our CurrentState so we can return to it
    (AI|Components|Blackboard|SetValueasEnum (Variables|Default|GetBlackboardReference) (Variables|BlackboardReferences|GetManualState) (Class|BlackboardComponent|GetValueasEnum (Variables|Default|GetBlackboardReference) (Variables|BlackboardReferences|GetCurrentState))))
  ;[1 1 1] Set NewState as CurrentState
  (AI|Components|Blackboard|SetValueasEnum (Variables|Default|GetBlackboardReference) (Variables|BlackboardReferences|GetCurrentState) (LocalVariables|GetLocalNewState))
  ;[1 1 1] Say we have a new State to switch to
  (AI|Components|Blackboard|SetValueasBool (Variables|Default|GetBlackboardReference) (Variables|BlackboardReferences|GetSetManualState) true)
  ;[1 1 1] Do we want to stop current MoveTo so it instantly starts new state
  (if (LocalVariables|GetLocalOverride)
    (CallFunction|CancelMoveto)))

(fn HowManyPlayersAreAlive
  (bind _array_element (Utilities|Array|ForEachLoopwithBreak (Variables|/Script/Engine.GameStateBase|GetPlayerArray (Game|GetGameState)))
    (:LoopBody
      (bind _asvert_player_state (Utilities|Casting|CastToVertPlayerState _array_element))
      (Utilities|IsValid (Pawn|GetControlledPawn (Class|VertPlayerState|GetController _asvert_player_state))
        (:Is%20Valid
          (Math|Integer|IncrementInt (LocalVariables|GetAliveActors)))))
    (:Completed
      (return (LocalVariables|GetAliveActors)))))

(fn StartupGorillaSequence
  (AI|RunBehaviorTree "/Game/AI/JoshAI/AI_Gorilla_BehaviorTree.AI_Gorilla_BehaviorTree")
  ;[1 1 1] Assign Blackboard Reference
  (bind _output_get (Variables|Default|SetBlackboardReference (AI|GetBlackboard self)))
  (Utilities|IsValid _output_get
    (:Is%20Valid
      ;[1 1 1] Assign BP_Gorilla Reference
      (bind _asbp_gorilla (Utilities|Casting|CastToBP_Gorilla (Pawn|GetControlledPawn (AI|GetAIController self)))
        (:then
          (bind _output_get_2 (Variables|References|SetBP_GorillaReference _asbp_gorilla))
          (Utilities|IsValid _output_get_2
            (:Is%20Valid
              (Development|PrintString "Setting Entry/Exit checkpoints")
              (AI|Components|Blackboard|SetValueasObject (Variables|Default|GetBlackboard) (Variables|BlackboardReferences|GetEntryCheckpoint) (Variables|/Game/AI/JoshAI/BP_Gorilla.BP_Gorilla_C|GetEntryCheckpoint (Variables|References|GetBP_GorillaReference)))
              (AI|Components|Blackboard|SetValueasObject (Variables|Default|GetBlackboard) (Variables|BlackboardReferences|GetExitCheckpoint) (Variables|/Game/AI/JoshAI/BP_Gorilla.BP_Gorilla_C|GetExitCheckpoint (Variables|References|GetBP_GorillaReference)))
              ;[1 1 1] Assign Starting State
              (AI|Components|Blackboard|SetValueasEnum (Variables|Default|GetBlackboard) (Variables|BlackboardReferences|GetCurrentState) (Utilities|Enum|LiteralenumEnum_Gorilla_AIState "NewEnumerator0")))))
        (:CastFailed
          (Development|PrintString "Cast to BP_Gorillar Failed"))))))