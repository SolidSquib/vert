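; Sky laser effect actor with two spark components, PSparksX and PSparksY, meant to slide along their local X and Y axes.
; BeginPlay caches both components' relative locations, and BeginPlay and EndPlay cast the game mode to VertGameMode.
; The four timelines that offset the sparks and the follow register/unregister calls are disconnected, so the sparks are never moved by this graph.
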(event EventBeginPlay
  (Variables|Default|SetSparks%20X+ (Variables|/Script/Engine.SceneComponent|GetRelativeLocation (Variables|Default|GetP_Sparks%20X+)))
  (Variables|Default|SetSparks%20X- (Variables|/Script/Engine.SceneComponent|GetRelativeLocation (Variables|Default|GetP_Sparks%20X-)))
  (Variables|Default|SetSparks%20Y+ (Variables|/Script/Engine.SceneComponent|GetRelativeLocation (Variables|Default|GetP_Sparks%20Y+)))
  (Variables|Default|SetSparks%20Y- (Variables|/Script/Engine.SceneComponent|GetRelativeLocation (Variables|Default|GetP_Sparks%20Y-)))
  (bind _asvert_game_mode (Utilities|Casting|CastToVertGameMode (Game|GetGameMode))))

(event EventEndPlay
  (params (EndPlayReason :type EEndPlayReason%20Enum :default "Destroyed"))
  (bind _asvert_game_mode (Utilities|Casting|CastToVertGameMode (Game|GetGameMode))))

(fn ConstructionScript)