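; Test camera drone actor that turns its skeletal mesh to face nearby VertCharacter pawns.
; Every tick it runs a debug-drawn multi-sphere trace around itself and rotates the mesh toward each matching hit.
; The look direction is rotated by a 90-degree offset, with pitch zeroed.
; A timeline bobbing motion around the location cached at BeginPlay exists but is never run.
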(event EventBeginPlay
  (Variables|Default|SetCamera_Drone (Variables|/Script/Engine.SceneComponent|GetRelativeLocation (Variables|Default|GetSK_Camera_Drone))))

(event EventTick
  (params (DeltaSeconds :type Float%20%28single-precision%29))
  (bind _returnvalue (Transformation|GetActorLocation))
  (bind _outhits (Collision|MultiSphereTraceForObjects _returnvalue _returnvalue 5e+03 (Utilities|Array|MakeArray "ObjectTypeQuery3") false 0 "ForOneFrame"))
  (bind _array_element (Utilities|Array|ForEachLoopwithBreak _outhits)
    (:LoopBody
      (Utilities|IsValid (.HitActor (Collision|BreakHitResult _array_element))
        (:Is%20Valid
          (Utilities|Casting|CastToVertCharacter (.HitActor (Collision|BreakHitResult _array_element)))
          (Transformation|SetWorldRotation (Variables|Default|GetSK_Camera_Drone) (Math|Rotator|MakeRotator (.Roll (Math|Rotator|BreakRotator (Math|Conversions|RotationFromXVector (Math|Vector|RotateVector (- (Transformation|GetActorLocation (.HitActor (Collision|BreakHitResult _array_element))) (Transformation|GetActorLocation)) "0.000000,-90.000000,0.000000")))) 0.0 (.Yaw (Math|Rotator|BreakRotator (Math|Conversions|RotationFromXVector (Math|Vector|RotateVector (- (Transformation|GetActorLocation (.HitActor (Collision|BreakHitResult _array_element))) (Transformation|GetActorLocation)) "0.000000,-90.000000,0.000000"))))) false false))))))

(fn ConstructionScript)