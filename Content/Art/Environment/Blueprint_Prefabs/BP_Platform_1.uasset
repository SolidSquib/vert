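; Environment prefab Blueprint of a platform with nine static mesh pieces, set up to float vertically as floating islands.
; BeginPlay caches each mesh's relative location as a base.
; Each mesh has its own Timeline that adds a Z offset to that base and sets the relative location without sweep.
; No Timeline play input is wired, so motion would depend on autoplay, which the graph does not show.
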(event EventBeginPlay
  (Variables|Default|SetNewVar_0 (Variables|/Script/Engine.SceneComponent|GetRelativeLocation (Variables|Default|GetStaticMeshComponent015)))
  (Variables|Default|SetNewVar_1 (Variables|/Script/Engine.SceneComponent|GetRelativeLocation (Variables|Default|GetStaticMeshComponent016)))
  (Variables|Default|SetNewVar_2 (Variables|/Script/Engine.SceneComponent|GetRelativeLocation (Variables|Default|GetStaticMeshComponent013)))
  (Variables|Default|SetNewVar_3 (Variables|/Script/Engine.SceneComponent|GetRelativeLocation (Variables|Default|GetStaticMeshComponent019)))
  (Variables|Default|SetNewVar_4 (Variables|/Script/Engine.SceneComponent|GetRelativeLocation (Variables|Default|GetStaticMeshComponent012)))
  (Variables|Default|SetNewVar_5 (Variables|/Script/Engine.SceneComponent|GetRelativeLocation (Variables|Default|GetStaticMeshComponent017)))
  (Variables|Default|SetNewVar_6 (Variables|/Script/Engine.SceneComponent|GetRelativeLocation (Variables|Default|GetStaticMeshComponent020)))
  (Variables|Default|SetNewVar_7 (Variables|/Script/Engine.SceneComponent|GetRelativeLocation (Variables|Default|GetStaticMeshComponent021)))
  (Variables|Default|SetNewVar_8 (Variables|/Script/Engine.SceneComponent|GetRelativeLocation (Variables|Default|GetStaticMeshComponent022))))

(fn ConstructionScript)