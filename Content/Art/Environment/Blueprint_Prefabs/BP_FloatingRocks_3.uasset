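; Environment prefab of eight floating rock meshes, built to bob vertically around their placed positions.
; BeginPlay caches each mesh's relative location as a base.
; Each mesh has its own Timeline whose track adds a Z offset to that base on update.
; Nothing in the graph triggers these Timelines, so the motion does not run from the logic shown.
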(event EventBeginPlay
  (Variables|Default|SetNewVar_0 (Variables|/Script/Engine.SceneComponent|GetRelativeLocation (Variables|Default|GetStaticMeshComponent0)))
  (Variables|Default|SetNewVar_1 (Variables|/Script/Engine.SceneComponent|GetRelativeLocation (Variables|Default|GetStaticMeshComponent01)))
  (Variables|Default|SetNewVar_2 (Variables|/Script/Engine.SceneComponent|GetRelativeLocation (Variables|Default|GetStaticMeshComponent02)))
  (Variables|Default|SetNewVar_3 (Variables|/Script/Engine.SceneComponent|GetRelativeLocation (Variables|Default|GetStaticMeshComponent03)))
  (Variables|Default|SetNewVar_4 (Variables|/Script/Engine.SceneComponent|GetRelativeLocation (Variables|Default|GetStaticMeshComponent04)))
  (Variables|Default|SetNewVar_5 (Variables|/Script/Engine.SceneComponent|GetRelativeLocation (Variables|Default|GetStaticMeshComponent05)))
  (Variables|Default|SetNewVar_6 (Variables|/Script/Engine.SceneComponent|GetRelativeLocation (Variables|Default|GetStaticMeshComponent06)))
  (Variables|Default|SetNewVar_7 (Variables|/Script/Engine.SceneComponent|GetRelativeLocation (Variables|Default|GetStaticMeshComponent07))))

(fn ConstructionScript)