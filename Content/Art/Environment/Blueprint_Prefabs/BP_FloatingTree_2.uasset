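; Floating tree environment prefab built to offset its meshes, petals component and two point lights vertically for a hovering motion.
; BeginPlay caches each component's relative location as a base.
; Each component has its own timeline whose float track adds a Z offset to that base on Update.
; The graph never calls Play on these timelines, so any motion would depend on autoplay settings not shown here.
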(event EventBeginPlay
  (Variables|Default|SetSM_01 (Variables|/Script/Engine.SceneComponent|GetRelativeLocation (Variables|Default|GetStaticMeshComponent01)))
  (Variables|Default|SetSM_02 (Variables|/Script/Engine.SceneComponent|GetRelativeLocation (Variables|Default|GetStaticMeshComponent02)))
  (Variables|Default|SetSM_03 (Variables|/Script/Engine.SceneComponent|GetRelativeLocation (Variables|Default|GetStaticMeshComponent03)))
  (Variables|Default|SetSM_04 (Variables|/Script/Engine.SceneComponent|GetRelativeLocation (Variables|Default|GetStaticMeshComponent04)))
  (Variables|Default|SetSM_05 (Variables|/Script/Engine.SceneComponent|GetRelativeLocation (Variables|Default|GetStaticMeshComponent05)))
  (Variables|Default|SetSM_06 (Variables|/Script/Engine.SceneComponent|GetRelativeLocation (Variables|Default|GetStaticMeshComponent06)))
  (Variables|Default|SetSM_07 (Variables|/Script/Engine.SceneComponent|GetRelativeLocation (Variables|Default|GetStaticMeshComponent07)))
  (Variables|Default|SetSM_08 (Variables|/Script/Engine.SceneComponent|GetRelativeLocation (Variables|Default|GetStaticMeshComponent08)))
  (Variables|Default|SetSM_09 (Variables|/Script/Engine.SceneComponent|GetRelativeLocation (Variables|Default|GetStaticMeshComponent09)))
  (Variables|Default|SetSM_0 (Variables|/Script/Engine.SceneComponent|GetRelativeLocation (Variables|Default|GetStaticMeshComponent0)))
  (Variables|Default|SetSM_11 (Variables|/Script/Engine.SceneComponent|GetRelativeLocation (Variables|Default|GetStaticMeshComponent011)))
  (Variables|Default|SetSM_12 (Variables|/Script/Engine.SceneComponent|GetRelativeLocation (Variables|Default|GetStaticMeshComponent012)))
  (Variables|Default|SetSM_13 (Variables|/Script/Engine.SceneComponent|GetRelativeLocation (Variables|Default|GetStaticMeshComponent013)))
  (Variables|Default|SetSM_14 (Variables|/Script/Engine.SceneComponent|GetRelativeLocation (Variables|Default|GetStaticMeshComponent014)))
  (Variables|Default|SetSM_15 (Variables|/Script/Engine.SceneComponent|GetRelativeLocation (Variables|Default|GetStaticMeshComponent015)))
  (Variables|Default|SetSM_16 (Variables|/Script/Engine.SceneComponent|GetRelativeLocation (Variables|Default|GetStaticMeshComponent016)))
  (Variables|Default|SetSM_A (Variables|/Script/Engine.SceneComponent|GetRelativeLocation (Variables|Default|GetStaticMesh)))
  (Variables|Default|SetSM_B (Variables|/Script/Engine.SceneComponent|GetRelativeLocation (Variables|Default|GetStaticMesh1)))
  (Variables|Default|SetPetals (Variables|/Script/Engine.SceneComponent|GetRelativeLocation (Variables|Default|GetP_Petals)))
  (Variables|Default|SetNewVar_0 (Variables|/Script/Engine.SceneComponent|GetRelativeLocation (Variables|Default|GetPointLight)))
  (Variables|Default|SetNewVar_1 (Variables|/Script/Engine.SceneComponent|GetRelativeLocation (Variables|Default|GetPointLight1))))

(fn ConstructionScript)