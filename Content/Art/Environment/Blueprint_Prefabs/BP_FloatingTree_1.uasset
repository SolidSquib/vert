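; Floating tree environment prefab, built to bob eight of its static mesh pieces vertically.
; BeginPlay caches each piece's relative location as a base position.
; Eight separate timelines each add a Z-only offset to that base through SetRelativeLocation on update.
; No event in the graph starts these timelines, so the bobbing does not run from the wiring shown.
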(event EventBeginPlay
  (Variables|Default|SetSM_01 (Variables|/Script/Engine.SceneComponent|GetRelativeLocation (Variables|Default|GetStaticMeshComponent01)))
  (Variables|Default|SetSM_02 (Variables|/Script/Engine.SceneComponent|GetRelativeLocation (Variables|Default|GetStaticMeshComponent02)))
  (Variables|Default|SetSM_04 (Variables|/Script/Engine.SceneComponent|GetRelativeLocation (Variables|Default|GetStaticMeshComponent04)))
  (Variables|Default|SetSM_05 (Variables|/Script/Engine.SceneComponent|GetRelativeLocation (Variables|Default|GetStaticMeshComponent05)))
  (Variables|Default|SetSM_06 (Variables|/Script/Engine.SceneComponent|GetRelativeLocation (Variables|Default|GetStaticMeshComponent06)))
  (Variables|Default|SetSM_07 (Variables|/Script/Engine.SceneComponent|GetRelativeLocation (Variables|Default|GetStaticMeshComponent07)))
  (Variables|Default|SetSM_08 (Variables|/Script/Engine.SceneComponent|GetRelativeLocation (Variables|Default|GetStaticMeshComponent0)))
  (Variables|Default|SetSM_09 (Variables|/Script/Engine.SceneComponent|GetRelativeLocation (Variables|Default|GetStaticMesh))))

(fn ConstructionScript)