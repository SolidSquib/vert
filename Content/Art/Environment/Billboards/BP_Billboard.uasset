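; BP_Billboard is an animated environment billboard that moves and flips on its own.
; On BeginPlay, a timeline lerps the skeletal billboard's relative location from StartLocation to EndLocation.
; In parallel, an endless delay loop alternates the flip and reverse-flip animations, with a longer wait before each flip than before each reversal.
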(event Collision|EventActorBeginOverlap
  (params (OtherActor :type Actor%20Object%20Reference)))

(event EventTick
  (params (DeltaSeconds :type Float%20%28single-precision%29)))

(event EventBeginPlay
  (Utilities|FlowControl|Sequence
    (:then_0
      (bind _newtrack_0 (Timeline|Timeline_0 Play)
        (:Update
          (Transformation|SetRelativeLocation (Variables|Default|GetSK_Billboard) (Math|Vector|Lerp(Vector) (Variables|Default|Getstart_Location) (Variables|Default|Getend%20location) _newtrack_0) false false))))
    (:then_1
      (Utilities|FlowControl|Delay 1e+01 :!label _label)
      (Components|Animation|PlayAnimation (Variables|Default|GetSK_Billboard) "/Game/Art/Environment/Billboards/Anim_Billboard_Flip.Anim_Billboard_Flip" false)
      (Utilities|FlowControl|Delay 5.0)
      (Components|Animation|PlayAnimation (Variables|Default|GetSK_Billboard) "/Game/Art/Environment/Billboards/Anim_Billboard_Flip_Reverse.Anim_Billboard_Flip_Reverse" false)
      (goto _label))))

(fn ConstructionScript)