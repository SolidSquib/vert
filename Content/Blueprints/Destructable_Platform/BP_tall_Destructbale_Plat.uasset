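; Tall destructible platform that can collapse when a Character steps onto its ledge collision.
; Each overlap rolls RNG against the current chance, and a failed roll raises that chance by a set increment, so collapse grows more likely with repeated visits.
; A successful roll waits an activation delay, then enables physics simulation on the rock mesh.
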(event OnComponentBeginOverlap(Ledge_Collision)
  (params (OverlappedComponent :type Primitive%20Component%20Object%20Reference) (OtherActor :type Actor%20Object%20Reference) (OtherComp :type Primitive%20Component%20Object%20Reference) (OtherBodyIndex :type Integer) (bFromSweep :type Boolean) (SweepResult :type Hit%20Result%20Structure%20%28by%20ref%29))
  (Utilities|Casting|CastToCharacter OtherActor)
  (bind _triggered (CallFunction|RNG (Variables|Default|GetCurrentChance)))
  (if _triggered
    (Utilities|FlowControl|Delay (Variables|Default|GetActivationDelay))
    (Physics|SetSimulatePhysics (Variables|Default|GetSM_Rock_11_DM) true)
    (else
      (Variables|Default|SetCurrentChance (+ (Variables|Default|GetCurrentChance) (Variables|Default|GetIncrementChance))))))

(event EventBeginPlay)

(event Collision|EventActorBeginOverlap
  (params (OtherActor :type Actor%20Object%20Reference)))

(event EventTick
  (params (DeltaSeconds :type Float%20%28single-precision%29)))

(fn ConstructionScript)