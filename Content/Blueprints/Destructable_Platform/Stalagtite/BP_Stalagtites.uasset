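; BP_Stalagtites is a falling stalactite hazard that damages and knocks back characters it hits.
; TriggerStalagtite enables physics on the skeletal mesh and marks it as falling.
; While falling, capsule overlaps with a Character apply point damage, stun and horizontal knockback away from the mesh.
; Overlapping a WorldStatic or WorldDynamic component clears the falling state and spawns a one-time impact particle at the FX socket.
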(event OnComponentBeginOverlap(SK_Stalagtite_m)
  (params (OverlappedComponent :type Primitive%20Component%20Object%20Reference) (OtherActor :type Actor%20Object%20Reference) (OtherComp :type Primitive%20Component%20Object%20Reference) (OtherBodyIndex :type Integer) (bFromSweep :type Boolean) (SweepResult :type Hit%20Result%20Structure%20%28by%20ref%29)))

(event OnComponentBeginOverlap(CapsuleCollider)
  (params (OverlappedComponent :type Primitive%20Component%20Object%20Reference) (OtherActor :type Actor%20Object%20Reference) (OtherComp :type Primitive%20Component%20Object%20Reference) (OtherBodyIndex :type Integer) (bFromSweep :type Boolean) (SweepResult :type Hit%20Result%20Structure%20%28by%20ref%29))
  (bind _returnvalue (Collision|GetCollisionObjectType OtherComp))
  (bind _returnvalue_2 (Transformation|GetActorLocation OtherActor))
  (bind _sk_stalagtite_m (Variables|Default|GetSK_Stalagtite_m))
  (bind _returnvalue_3 (Transformation|GetWorldLocation _sk_stalagtite_m))
  (bind _returnvalue_4 (- _returnvalue_2 _returnvalue_3))
  (bind (_x _y) (Math|Vector|BreakVector _returnvalue_4))
  (if (or (Utilities|Enum|Equal(Enum) _returnvalue "ECC_WorldDynamic") (Utilities|Enum|Equal(Enum) _returnvalue "ECC_WorldStatic"))
    (Development|PrintString "StaticDynamic")
    (Variables|Default|SetIsFalling false)
    (Utilities|FlowControl|DoOnce false
      (:Completed
        (Effects|SpawnEmitteratLocation "/Game/Art/Particles/P_HammerImpact.P_HammerImpact" (Transformation|GetSocketLocation (Variables|Default|GetSK_Stalagtite_m) "FXSocket"))))
    (else
      (bind _ascharacter (Utilities|Casting|CastToCharacter OtherActor))
      (if (Variables|Default|GetIsFalling)
        (Class|VertUtilities|VERTTakePointDamage _ascharacter (Variables|Default|GetDamage) "/Game/Blueprints/Weapons/DamageTypes/DamageTaken/BP_DamageType_Taken_ForgeHammer.BP_DamageType_Taken_ForgeHammer_C" (Math|Vector|Normalize (Math|Vector|MakeVector _x _y 0.0)) SweepResult (Variables|Default|GetKnockback) 1.0 0.5 (Game|GetInstigatorController) self)))))

(fn ConstructionScript)

(fn TriggerStalagtite
  (Physics|SetSimulatePhysics (Variables|Default|GetSK_Stalagtite_m) true)
  (Variables|Default|SetIsFalling true))