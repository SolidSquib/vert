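; BP_Stalagtite_Trigger is a trigger volume that sets off linked stalagtites by chance when a Character enters it.
; Each overlap rolls RNG against CurrentChance, and a failed roll raises that chance by Incrementchance for later entries.
; A successful roll calls TriggerStalagtite on every BP_Stalagtites in the Stalagtites array, then destroys the trigger so it fires only once.
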(event OnComponentBeginOverlap(Box_Stalagtite_Trigger)
  (params (OverlappedComponent :type Primitive%20Component%20Object%20Reference) (OtherActor :type Actor%20Object%20Reference) (OtherComp :type Primitive%20Component%20Object%20Reference) (OtherBodyIndex :type Integer) (bFromSweep :type Boolean) (SweepResult :type Hit%20Result%20Structure%20%28by%20ref%29))
  (Utilities|Casting|CastToCharacter OtherActor)
  (bind _triggered (CallFunction|RNG (Variables|Default|GetCurrentChance)))
  (if _triggered
    (bind _array_element (Utilities|Array|ForEachLoopwithBreak (Variables|Default|GetStalagtites))
      (:LoopBody
        (bind _asbp_stalagtites (Utilities|Casting|CastToBP_Stalagtites _array_element))
        (Default|TriggerStalagtite _asbp_stalagtites))
      (:Completed
        (Actor|DestroyActor)))
    (else
      (Variables|Default|SetCurrentChance (+ (Variables|Default|GetCurrentChance) (Variables|Default|GetIncrementchance))))))

(fn ConstructionScript)