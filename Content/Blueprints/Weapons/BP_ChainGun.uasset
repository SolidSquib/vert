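; Chain gun weapon Blueprint that must wind up while attack is held before it fires.
; After the delay, a FireWeapon flag unlocks the parent's attack and client simulation, slows the owner to walk speed and plays the firing animation.
; A looping-sound state starts fire audio once and posts a stop event on release or empty clip.
; Releasing or throwing the weapon restores the owner's starting move speed.
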(event EventBeginPlay
  (Actor|Tick|SetActorTickEnabled true))

(event Collision|EventActorBeginOverlap
  (params (OtherActor :type Actor%20Object%20Reference)))

(event EventWeaponReadyfromPickup
  ;[1 1 1] Assign CharacterMovement Reference and set Local RunSpeed
  (Variables|Default|SetAttackHeldDown false)
  (Variables|Default|SetFireWeapon false))

(event EventEVENTonPoolBeginPlay
  (Actor|Tick|SetActorTickEnabled true))

(event EventTick
  (params (DeltaSeconds :type Float%20%28single-precision%29))
  (if (Variables|Default|GetAttackHeldDown)
    (if (and (== (Class|BaseWeapon|GetCurrentAmmoinClip) 0) (== (Variables|Default|GetCurrentSound) (Variables|Default|GetFireSound)))
      (bind _output_get (Variables|Default|SetCurrentSound (Variables|Default|GetFireStopSound)))
      (Utilities|IsValid _output_get
        (:Is%20Valid
          (Class|AkGameplayStatics|PostEvent (Variables|Default|GetCurrentSound) self true)
          (Variables|Default|SetPlayingSound true))))))

(event EventOnStartAttacking
  (bind _returnvalue (Class|BaseWeapon|GetPawnOwner))
  (bind _weaponmesh (Variables|Default|GetWeaponMesh))
  (if (Utilities|IsValid _returnvalue)
    ;[1 1 1] AttackButtonDown - Shoot gun
    (Variables|Default|SetAttackHeldDown true)
    (Utilities|FlowControl|Delay (Variables|Default|GetWindUpDuration))
    (if (Variables|Default|GetAttackHeldDown)
      (|CallParentFunction)
      (Variables|Default|SetFireWeapon true)
      (Variables|/Script/Engine.CharacterMovementComponent|SetMaxWalkSpeed (Variables|/Script/Engine.Character|GetCharacterMovement _returnvalue) (Variables|Default|GetWalkSpeed))
      (Components|Timeline|SetPlayRate _weaponmesh 1.0)
      (Components|Animation|PlayAnimation _weaponmesh "/Game/Art/Weapons/Chaingun/Anim_Chaingun_Firing.Anim_Chaingun_Firing" false))))

(event EventOnStopAttacking
  (params (forced :type Boolean))
  (bind _returnvalue (Class|BaseWeapon|GetPawnOwner))
  (bind _firestopsound (Variables|Default|GetFireStopSound))
  ;[1 1 1] Comment
  (|CallParentFunction forced)
  (Variables|Default|SetAttackHeldDown false)
  (Variables|Default|SetFireWeapon false)
  (Utilities|FlowControl|Sequence
    (:then_0
      (Utilities|IsValid _returnvalue
        (:Is%20Valid
          (Variables|/Script/Engine.CharacterMovementComponent|SetMaxWalkSpeed (Variables|/Script/Engine.Character|GetCharacterMovement _returnvalue) (Class|VertCharacter|GetStartingMaxMoveSpeed _returnvalue))
          (Components|Timeline|SetPlayRate (Variables|Default|GetWeaponMesh) 0.5)
          (Utilities|FlowControl|Delay 0.2)
          (Audio|Components|Audio|Stop (Variables|Default|GetWeaponMesh)))))
    (:then_1
      (if (Variables|Default|GetPlayingSound)
        (Utilities|IsValid _firestopsound
          (:Is%20Valid
            (Class|AkGameplayStatics|PostEvent _firestopsound self false)
            (Variables|Default|SetPlayingSound false)))))))

(event EventThrowWeapon
  (bind _returnvalue (Class|BaseWeapon|GetPawnOwner))
  ;[1 1 1] Comment
  (if (Utilities|IsValid _returnvalue)
    (Variables|/Script/Engine.CharacterMovementComponent|SetMaxWalkSpeed (Variables|/Script/Engine.Character|GetCharacterMovement _returnvalue) (Class|VertCharacter|GetStartingMaxMoveSpeed _returnvalue))
    (|CallParentFunction)))

(event EventClientSimulateWeaponAttack
  ;[1 1 1] Stops Attack Call until its actually shooting (Also stops MuzzleFlash being early)
  (if (Variables|Default|GetFireWeapon)
    (|CallParentFunction)))

(fn ConstructionScript)

(fn AttackwithWeapon
  (if (Variables|Default|GetFireWeapon)
    (|CallParentFunction)
    (Variables|Default|SetCurrentSound (Variables|Default|GetFireSound))
    (Utilities|IsValid (Variables|Default|GetCurrentSound)
      (:Is%20Valid
        (if (not (Variables|Default|GetPlayingSound))
          (Class|AkGameplayStatics|PostEvent (Variables|Default|GetCurrentSound) self true)
          (Variables|Default|SetPlayingSound true)))
      (:Is%20Not%20Valid
        _))
    (return true)))

(fn EmptyFunction)