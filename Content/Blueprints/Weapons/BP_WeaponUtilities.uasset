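; Weapon utility Blueprint providing a melee trace that damages actors along a weapon socket's path.
; Each call sphere-sweeps from the last position, or the current socket on a new trace, to the current socket, with one-frame debug drawing.
; Newly hit actors receive VERT point damage with upward-biased knockback and stun from weapon data, plus impact particles and Wwise audio.
; It returns position and hit list for chaining calls without repeat hits.
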(fn MeleeWeaponTrace
  (params (Attach%20To%20Component :type Primitive%20Component%20Object%20Reference) (Attach%20Socket%20Name :type Name) (Start%20New%20Trace :type Boolean) (Last%20Trace%20Position :type Vector) (Trace%20Radius :type Float%20%28single-precision%29) (Trace%20Channel :type ETraceTypeQuery%20Enum) (Actors%20To%20Ignore :type Array%20of%20Actor%20Object%20References) (Weapon%20Data :type Weapon%20Data%20Structure) (Event%20Instigator :type Controller%20Object%20Reference) (Damage%20Causer :type Actor%20Object%20Reference) (Impact%20Particle%20Template :type Particle%20System%20Object%20Reference) (Impact%20Audio%20Event :type Ak%20Audio%20Event%20Object%20Reference))
  (bind (_infiniteammo _infiniteclip _ammoperclip _initialclips _basedamage _damagetype _timebetweenshots _firingmode _burstnumberofshots _bursttimebetweenshots _baseknockback _knockbackscaling _stuntime) (Utilities|Struct|BreakWeaponData Weapon%20Data))
  (bind _returnvalue (Transformation|GetSocketLocation Attach%20To%20Component Attach%20Socket%20Name))
  (Utilities|IsValid Attach%20To%20Component
    (:Is%20Valid
      (if Start%20New%20Trace
        (LocalVariables|SetFrom%20Trace%20Position _returnvalue)
        (else
          (LocalVariables|SetFrom%20Trace%20Position Last%20Trace%20Position)))
      (bind _output_get (LocalVariables|SetOut%20Hit%20Actors Actors%20To%20Ignore))
      (bind _output_get_2 (LocalVariables|SetTo%20Trace%20Position _returnvalue))
      (bind _outhits (Collision|MultiSphereTraceByChannel Attach%20To%20Component (LocalVariables|GetFrom%20Trace%20Position) _output_get_2 Trace%20Radius Trace%20Channel false _output_get "ForOneFrame"))
      (bind _array_element (Utilities|Array|ForEachLoopwithBreak _outhits)
        (:LoopBody
          (if (not (Utilities|Array|ContainsItem _output_get (.HitActor (Collision|BreakHitResult _array_element))))
            (Class|VertUtilities|VERTTakePointDamage (.HitActor (Collision|BreakHitResult _array_element)) (Math|Conversions|ToFloat(Integer) _basedamage) _damagetype (Math|Vector|Normalize (+ (- (.ImpactPoint (Collision|BreakHitResult _array_element)) (Transformation|GetWorldLocation Attach%20To%20Component)) (Math|Vector|MakeVector 0.0 0.0 1.0))) _array_element _baseknockback _knockbackscaling _stuntime Event%20Instigator Damage%20Causer)
            (Utilities|Array|AddUnique (LocalVariables|GetOut%20Hit%20Actors) (.HitActor (Collision|BreakHitResult _array_element)))
            (Utilities|IsValid Impact%20Particle%20Template
              (:Is%20Valid
                (Effects|SpawnEmitteratLocation (.HitActor (Collision|BreakHitResult _array_element)) Impact%20Particle%20Template (.ImpactPoint (Collision|BreakHitResult _array_element))))
              (:Is%20Not%20Valid
                _))
            (Utilities|IsValid 0
              (:Is%20Valid
                (Class|AkGameplayStatics|PostEvent Impact%20Audio%20Event (.HitActor (Collision|BreakHitResult _array_element)) true)))))
        (:Completed
          (return (LocalVariables|GetTo%20Trace%20Position) (LocalVariables|GetOut%20Hit%20Actors) true))))
    (:Is%20Not%20Valid
      (return "0, 0, 0" 0 false))))