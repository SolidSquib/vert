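; Default unarmed weapon: a hold-to-charge punch that cannot be picked up.
; Holding attack sets walk speed, accrues capped damage and knockback on a Tick timer, and ramps fist particles and rumble via timeline.
; Release passes a punch impulse to the character and sphere-sweeps the right hand between frames, damaging each actor once.
; Attacks pressed during lockout are buffered and retried on Tick; forced stops reset all state.
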(event EventBeginPlay
  ;[1 1 1] Never allow interaction on a default weapon
  (Class|Interactive|DisableInteractionDetection))

(event Collision|EventActorBeginOverlap
  (params (OtherActor :type Actor%20Object%20Reference)))

(event EventTick
  (params (DeltaSeconds :type Float%20%28single-precision%29))
  (bind _returnvalue (Class|BaseWeapon|GetPawnOwner))
  (bind _returnvalue_2 (Class|BaseWeapon|GetPawnOwner))
  (Utilities|FlowControl|Sequence
    (:then_0
      (CallFunction|WeaponHitTracing))
    (:then_1
      ;[1 1 1] A Timer for Calling ChargeWeapon
      (Variables|Default|SetTimer (+ (Variables|Default|GetTimer) DeltaSeconds))
      (if (>= (Variables|Default|GetTimer) 0.1)
        (Variables|Default|SetTimer 0.0)
        (CallFunction|ChargeWeapon)))
    (:then_2
      (if (Variables|Default|GetClipAnimations)
        (if (Variables|Default|GetLockWeaponInput)
          (Variables|Default|SetClipAnimations true)
          (else
            (Variables|Default|SetClipAnimations false)
            (|CallParentFunction)
            (Class|MeleeWeapon|ResetComboDepth)
            (Class|BaseWeapon|ResetBonusDamageandKnockback)
            (Variables|Default|SetWeaponRaised true)
            (Utilities|IsValid _returnvalue_2
              (:Is%20Valid
                (Variables|/Script/Engine.CharacterMovementComponent|SetMaxWalkSpeed (Variables|/Script/Engine.Character|GetCharacterMovement _returnvalue_2) (Variables|Default|GetWalkSpeed))
                (Class|BaseWeapon|WeaponAttackFire 0.0) ; Trigger Combo_0
                (Utilities|FlowControl|Sequence
                  (:then_0
                    (if (Utilities|IsValid _returnvalue)
                      ;[1 0.2602 0.9711] Spawn Fist FX and saving as local variable
                      (bind _returnvalue_3 (Effects|SpawnEmitterAttached "/Game/Art/Particles/P_PlayerFist.P_PlayerFist" (Variables|/Script/Engine.Character|GetMesh _returnvalue) "RightHand_Socket" "0, 0, 0" "0, 0,0.000000" "SnapToTargetIncludingScale"))
                      (Variables|Default|SetFistParticle _returnvalue_3)
                      (Utilities|IsValid (Variables|Default|GetFistParticle)
                        (:Is%20Valid
                          (Components|Timeline|SetPlayRate (Variables|Default|GetBlend_FistFXValues) 1.0) ; Default is 1 second
                          ;[0.3755 0.1074 0.555] Setting Fist Size and Colour based on Lerp values
                          (bind _smoothlerp (Timeline|Blend_FistFXValues PlayFromStart)
                            (:Update
                              (Utilities|FlowControl|Sequence
                                (:then_0
                                  (if (Utilities|IsValid (Variables|Default|GetFistParticle))
                                    (Utilities|FlowControl|Sequence
                                      (:then_0
                                        (Effects|Components|ParticleSystem|SetVectorParameter (Variables|Default|GetFistParticle) "PlayerFist_Size" (Math|Vector|MakeVector (Math|Float|Lerp 0.8 1.0 _smoothlerp) (Math|Float|Lerp 0.8 1.0 _smoothlerp) (Math|Float|Lerp 0.8 1.0 _smoothlerp))))
                                      (:then_1
                                        (Effects|Components|ParticleSystem|SetVectorParameter (Variables|Default|GetFistParticle) "PlayerFist_Col" (Math|Vector|Lerp(Vector) (Variables|Default|GetFX_StartingColour) (Variables|Default|GetFX_EndColour) _smoothlerp))))
                                    (else
                                      (Timeline|Blend_FistFXValues Stop))))
                                (:then_1
                                  (Utilities|GetValidPlayerController
                                    (:Valid%20Controller
                                      (goto _label Update))))
                                (:then_2
                                  (Effects|Components|ParticleSystem|SetVectorParameter (Variables|Default|GetFistParticle) "PlayerFist_Speed" (Math|Vector|MakeVector 0.0 (Math|Float|Lerp -1.0 -3.0 _smoothlerp) 0.0))))))))))
                  (:then_1
                    ;[1 0.1972 0] Set Charging Forcefeedback
                    (Utilities|GetValidPlayerController
                      (:Valid%20Controller
                        (Game|Feedback|PlayDynamicForceFeedback (Variables|Default|GetPlayerController) (Math|Float|Lerp 0.0 0.3 _smoothlerp) -1.0 false false false true :!label _label)))))))))))))

(event EventNotifyAttackAnimationEnded
  (bind _returnvalue (Class|BaseWeapon|GetPawnOwner))
  (bind _fistparticle (Variables|Default|GetFistParticle))
  (|CallParentFunction)
  (Variables|HitTracing|SetStartHitTracing false)
  (if (Utilities|IsValid _returnvalue)
    (Utilities|FlowControl|Sequence
      (:then_0
        (Variables|/Script/Engine.CharacterMovementComponent|SetMaxWalkSpeed (Variables|/Script/Engine.Character|GetCharacterMovement _returnvalue) (Class|VertCharacter|GetStartingMaxMoveSpeed _returnvalue)))
      (:then_1
        (Utilities|GetValidPlayerController
          (:Valid%20Controller
            (Game|Feedback|PlayDynamicForceFeedback (Variables|Default|GetPlayerController) (Math|Float|Lerp 0.0 0.3 (stale _smoothlerp)) -1.0 false false false true) ; enters at Stop
          )))
      (:then_2
        (Utilities|Array|Clear (Variables|HitTracing|GetHitArray))
        ;[1 0.2602 0.9711] Destroy FX
        (if (Utilities|IsValid _fistparticle)
          (Audio|Components|Audio|Stop (Variables|Default|GetBlend_FistFXValues)))
        (Components|DestroyComponent _fistparticle)
        (Utilities|FlowControl|Sequence
          (:then_0
            ;[0.3755 0.1074 0.555] Setting Fist Size and Colour based on Lerp values
            (bind _smoothlerp (Timeline|Blend_FistFXValues Stop)
              (:Update
                (Utilities|FlowControl|Sequence
                  (:then_0
                    (if (Utilities|IsValid (Variables|Default|GetFistParticle))
                      (Utilities|FlowControl|Sequence
                        (:then_0
                          (Effects|Components|ParticleSystem|SetVectorParameter (Variables|Default|GetFistParticle) "PlayerFist_Size" (Math|Vector|MakeVector (Math|Float|Lerp 0.8 1.0 _smoothlerp) (Math|Float|Lerp 0.8 1.0 _smoothlerp) (Math|Float|Lerp 0.8 1.0 _smoothlerp))))
                        (:then_1
                          (Effects|Components|ParticleSystem|SetVectorParameter (Variables|Default|GetFistParticle) "PlayerFist_Col" (Math|Vector|Lerp(Vector) (Variables|Default|GetFX_StartingColour) (Variables|Default|GetFX_EndColour) _smoothlerp))))
                      (else
                        (Timeline|Blend_FistFXValues Stop))))
                  (:then_1
                    (Utilities|GetValidPlayerController
                      (:Valid%20Controller
                        (Game|Feedback|PlayDynamicForceFeedback (Variables|Default|GetPlayerController) (Math|Float|Lerp 0.0 0.3 _smoothlerp) -1.0 false false false true) ; enters at Update
                      )))
                  (:then_2
                    (Effects|Components|ParticleSystem|SetVectorParameter (Variables|Default|GetFistParticle) "PlayerFist_Speed" (Math|Vector|MakeVector 0.0 (Math|Float|Lerp -1.0 -3.0 _smoothlerp) 0.0)))))))
          (:then_1
            (Utilities|FlowControl|Delay (Variables|Default|GetLockoutDelay))
            (Variables|Default|SetLockWeaponInput false)))))))

(event EventWeaponReadyfromPickup
  (Development|PrintString "Unarmed Ready for Pickup" false false))

(event EventOnStartAttacking
  (bind _returnvalue (Class|BaseWeapon|GetPawnOwner))
  (bind _returnvalue_2 (Class|BaseWeapon|GetPawnOwner))
  (if (Variables|Default|GetLockWeaponInput)
    (Variables|Default|SetClipAnimations true)
    (else
      (Variables|Default|SetClipAnimations false)
      (|CallParentFunction)
      (Class|MeleeWeapon|ResetComboDepth)
      (Class|BaseWeapon|ResetBonusDamageandKnockback)
      (Variables|Default|SetWeaponRaised true)
      (Utilities|IsValid _returnvalue_2
        (:Is%20Valid
          (Variables|/Script/Engine.CharacterMovementComponent|SetMaxWalkSpeed (Variables|/Script/Engine.Character|GetCharacterMovement _returnvalue_2) (Variables|Default|GetWalkSpeed))
          (Class|BaseWeapon|WeaponAttackFire 0.0) ; Trigger Combo_0
          (Utilities|FlowControl|Sequence
            (:then_0
              (if (Utilities|IsValid _returnvalue)
                ;[1 0.2602 0.9711] Spawn Fist FX and saving as local variable
                (bind _returnvalue_3 (Effects|SpawnEmitterAttached "/Game/Art/Particles/P_PlayerFist.P_PlayerFist" (Variables|/Script/Engine.Character|GetMesh _returnvalue) "RightHand_Socket" "0, 0, 0" "0, 0,0.000000" "SnapToTargetIncludingScale"))
                (Variables|Default|SetFistParticle _returnvalue_3)
                (Utilities|IsValid (Variables|Default|GetFistParticle)
                  (:Is%20Valid
                    (Components|Timeline|SetPlayRate (Variables|Default|GetBlend_FistFXValues) 1.0) ; Default is 1 second
                    ;[0.3755 0.1074 0.555] Setting Fist Size and Colour based on Lerp values
                    (bind _smoothlerp (Timeline|Blend_FistFXValues PlayFromStart)
                      (:Update
                        (Utilities|FlowControl|Sequence
                          (:then_0
                            (if (Utilities|IsValid (Variables|Default|GetFistParticle))
                              (Utilities|FlowControl|Sequence
                                (:then_0
                                  (Effects|Components|ParticleSystem|SetVectorParameter (Variables|Default|GetFistParticle) "PlayerFist_Size" (Math|Vector|MakeVector (Math|Float|Lerp 0.8 1.0 _smoothlerp) (Math|Float|Lerp 0.8 1.0 _smoothlerp) (Math|Float|Lerp 0.8 1.0 _smoothlerp))))
                                (:then_1
                                  (Effects|Components|ParticleSystem|SetVectorParameter (Variables|Default|GetFistParticle) "PlayerFist_Col" (Math|Vector|Lerp(Vector) (Variables|Default|GetFX_StartingColour) (Variables|Default|GetFX_EndColour) _smoothlerp))))
                              (else
                                (Timeline|Blend_FistFXValues Stop))))
                          (:then_1
                            (Utilities|GetValidPlayerController
                              (:Valid%20Controller
                                (goto _label Update))))
                          (:then_2
                            (Effects|Components|ParticleSystem|SetVectorParameter (Variables|Default|GetFistParticle) "PlayerFist_Speed" (Math|Vector|MakeVector 0.0 (Math|Float|Lerp -1.0 -3.0 _smoothlerp) 0.0))))))))))
            (:then_1
              ;[1 0.1972 0] Set Charging Forcefeedback
              (Utilities|GetValidPlayerController
                (:Valid%20Controller
                  (Game|Feedback|PlayDynamicForceFeedback (Variables|Default|GetPlayerController) (Math|Float|Lerp 0.0 0.3 _smoothlerp) -1.0 false false false true :!label _label))))))))))

(event EventOnStopAttacking
  (params (forced :type Boolean))
  (bind _returnvalue (Class|BaseWeapon|GetPawnOwner))
  (bind _returnvalue_2 (Class|BaseWeapon|GetPawnOwner))
  (bind _fistparticle (Variables|Default|GetFistParticle))
  (Variables|Default|SetClipAnimations false)
  (if forced
    (CallFunction|ResetAttackStates)
    (Utilities|FlowControl|Sequence
      (:then_0
        (Utilities|GetValidPlayerController :!label _label
          (:Valid%20Controller
            (Game|Feedback|PlayDynamicForceFeedback (Variables|Default|GetPlayerController) (Math|Float|Lerp 0.0 0.3 (stale _smoothlerp)) -1.0 false false false true) ; enters at Stop
          )))
      (:then_1
        ;[0.3755 0.1074 0.555] Setting Fist Size and Colour based on Lerp values
        (bind _smoothlerp (Timeline|Blend_FistFXValues Stop)
          (:Update
            (Utilities|FlowControl|Sequence
              (:then_0
                (if (Utilities|IsValid (Variables|Default|GetFistParticle))
                  (Utilities|FlowControl|Sequence
                    (:then_0
                      (Effects|Components|ParticleSystem|SetVectorParameter (Variables|Default|GetFistParticle) "PlayerFist_Size" (Math|Vector|MakeVector (Math|Float|Lerp 0.8 1.0 _smoothlerp) (Math|Float|Lerp 0.8 1.0 _smoothlerp) (Math|Float|Lerp 0.8 1.0 _smoothlerp))))
                    (:then_1
                      (Effects|Components|ParticleSystem|SetVectorParameter (Variables|Default|GetFistParticle) "PlayerFist_Col" (Math|Vector|Lerp(Vector) (Variables|Default|GetFX_StartingColour) (Variables|Default|GetFX_EndColour) _smoothlerp))))
                  (else
                    (Timeline|Blend_FistFXValues Stop))))
              (:then_1
                (Utilities|GetValidPlayerController
                  (:Valid%20Controller
                    (Game|Feedback|PlayDynamicForceFeedback (Variables|Default|GetPlayerController) (Math|Float|Lerp 0.0 0.3 _smoothlerp) -1.0 false false false true) ; enters at Update
                  )))
              (:then_2
                (Effects|Components|ParticleSystem|SetVectorParameter (Variables|Default|GetFistParticle) "PlayerFist_Speed" (Math|Vector|MakeVector 0.0 (Math|Float|Lerp -1.0 -3.0 _smoothlerp) 0.0)))))))
      (:then_2
        (if (Utilities|IsValid _fistparticle)
          (Components|DestroyComponent _fistparticle))))
    (else
      (Utilities|FlowControl|Sequence
        (:then_0
          (if (Variables|Default|GetWeaponRaised)
            (Variables|Default|SetLockWeaponInput true)
            (Variables|Default|SetWeaponRaised false)
            (if (Utilities|IsValid _returnvalue_2)
              (Variables|/Script/Engine.CharacterMovementComponent|SetMaxWalkSpeed (Variables|/Script/Engine.Character|GetCharacterMovement _returnvalue_2) (Class|VertCharacter|GetStartingMaxMoveSpeed _returnvalue_2))
              (if (Utilities|IsValid _returnvalue)
                (bind _asbp_vert_character (Utilities|Casting|CastToBP_VertCharacter _returnvalue)
                  (:then
                    (Default|PassPunchImpulse _asbp_vert_character (Math|Float|NormalizetoRange (Class|BaseWeapon|GetBonusKnockback) 0.0 (Variables|ChargeValues|GetMaxBonusKnockback))))
                  (:CastFailed
                    _))
                (Class|MeleeWeapon|IncrementComboDepth) ; So it plays Combo_1 Attack
                (Class|BaseWeapon|WeaponAttackFire 0.0)
                (Variables|HitTracing|SetStartHitTracing true)
                (Variables|HitTracing|SetSetStartingTracePosition true)
                (Utilities|FlowControl|Sequence
                  (:then_0
                    ;[1 0.7768 0] Play Audio
                    (Class|AkGameplayStatics|PostEvent (Variables|Default|GetPunchSwingSound) (Class|BaseWeapon|GetPawnOwner) true))
                  (:then_1
                    ;[1 0.1972 0] Set Firing Forcefeedback
                    (if (Utilities|IsValid (Class|BaseWeapon|GetPawnOwner))
                      _)))))))
        (:then_1
          (goto _label))))))

(fn ConstructionScript)

(fn ChargeWeapon
  (if (Variables|Default|GetWeaponRaised)
    (Class|BaseWeapon|AddBonusDamageandKnockback (Math|Integer|SelectInt (Variables|ChargeValues|GetBonusDamageIncrementAmount) 0 (< (Class|BaseWeapon|GetBonusDamage) (Variables|ChargeValues|GetMaxBonusDamageAmount))) (Math|Float|SelectFloat (Variables|ChargeValues|GetBonusKnockbackIncrementAmount) 0.0 (< (Class|BaseWeapon|GetBonusKnockback) (Variables|ChargeValues|GetMaxBonusKnockback)))))
  (return))

(fn AttackwithWeapon
  (return false) ; True to consume Ammo and Play Audio
)

(fn WeaponHitTracing
  (if (Variables|HitTracing|GetStartHitTracing)
    (CallFunction|HandTrace (Variables|HitTracing|GetRightHandSocket))
    (else
      (return))))

(fn ResetAttackStates
  (bind _returnvalue (Class|BaseWeapon|GetPawnOwner))
  (bind _returnvalue_2 (Class|BaseWeapon|GetPawnOwner))
  (bind _fistparticle (Variables|Default|GetFistParticle))
  (if (Utilities|IsValid _returnvalue)
    (Utilities|FlowControl|Sequence
      (:then_0
        (|CallParentFunction)
        (Variables|HitTracing|SetStartHitTracing false)
        (Variables|Default|SetLockWeaponInput false)
        (Variables|Default|SetWeaponRaised false)
        (Variables|Default|SetClipAnimations false)
        (Variables|/Script/Engine.CharacterMovementComponent|SetMaxWalkSpeed (Variables|/Script/Engine.Character|GetCharacterMovement _returnvalue) (Class|VertCharacter|GetStartingMaxMoveSpeed _returnvalue))
        (Class|MeleeWeapon|ResetComboDepth)
        (Class|BaseWeapon|ResetBonusDamageandKnockback)
        (Utilities|Array|Clear (Variables|HitTracing|GetHitArray))
        ;[0.3755 0.1074 0.555] Add Stop to particles
        (if (Utilities|IsValid _fistparticle)
          (Components|DestroyComponent _fistparticle)))
      (:then_1
        (bind _asbp_vert_animation (Utilities|Casting|CastToBP_VertAnimation (Components|SkeletalMesh|GetAnimInstance (Variables|/Script/Engine.Character|GetMesh _returnvalue))))
        (Default|ResettoIdle _asbp_vert_animation))
      (:then_2
        (if (Utilities|IsValid _returnvalue_2)
          (bind _asplayer_controller (Utilities|Casting|CastToPlayerController (Pawn|GetController _returnvalue_2)))
          (Game|Feedback|ClientStopForceFeedback _asplayer_controller 0 "Firing")))
      (:then_3
        (return)))))

(fn HandTrace
  (params (WhichHand :type Name))
  (bind _returnvalue (Class|BaseWeapon|GetPawnOwner))
  (bind _weaponconfig (Variables|Default|GetWeaponConfig))
  (bind (_basedamage _damagetype _timebetweenshots _firingmode _burstnumberofshots _bursttimebetweenshots _baseknockback _knockbackscaling _stuntime) (Utilities|Struct|BreakWeaponData _weaponconfig))
  (LocalVariables|SetLocalSocketlocation (Transformation|GetSocketLocation (Variables|/Script/Engine.Character|GetMesh (Class|BaseWeapon|GetPawnOwner)) WhichHand))
  (if (Variables|HitTracing|GetSetStartingTracePosition)
    (Variables|HitTracing|SetLastHitTracePosition (LocalVariables|GetLocalSocketlocation))
    (Variables|HitTracing|SetSetStartingTracePosition false)
    (else
      (Variables|HitTracing|SetLastHitTracePosition (Variables|HitTracing|GetNewHitTracePosition))))
  (Variables|HitTracing|SetNewHitTracePosition (LocalVariables|GetLocalSocketlocation))
  (bind _outhits (Collision|MultiSphereTraceByChannel (Variables|HitTracing|GetLastHitTracePosition) (Variables|HitTracing|GetNewHitTracePosition) 5e+01 "TraceTypeQuery5" false (Utilities|Array|MakeArray (Class|BaseWeapon|GetPawnOwner)) "None"))
  (bind _array_element (Utilities|Array|ForEachLoopwithBreak _outhits)
    (:LoopBody
      (if (== (Utilities|Array|FindItem (Variables|HitTracing|GetHitArray) (.HitActor (Collision|BreakHitResult _array_element))) -1)
        (Class|VertUtilities|VERTTakePointDamage (.HitActor (Collision|BreakHitResult _array_element)) (Math|Conversions|ToFloat(Integer) (+ _basedamage (Class|BaseWeapon|GetBonusDamage))) _damagetype (Math|Vector|MakeVectorNetQuantizeNormal (.X (Math|Vector|BreakVector (Math|Vector|Normalize (- (.TraceEnd (Collision|BreakHitResult _array_element)) (.TraceStart (Collision|BreakHitResult _array_element)))))) (.Y (Math|Vector|BreakVector (Math|Vector|Normalize (- (.TraceEnd (Collision|BreakHitResult _array_element)) (.TraceStart (Collision|BreakHitResult _array_element)))))) (.Z (Math|Vector|BreakVector (Math|Vector|Normalize (- (.TraceEnd (Collision|BreakHitResult _array_element)) (.TraceStart (Collision|BreakHitResult _array_element))))))) _array_element (+ _baseknockback (Class|BaseWeapon|GetBonusKnockback)) _knockbackscaling _stuntime (Pawn|GetController (Variables|Default|GetInstigator)) self)
        (Utilities|Array|AddUnique (Variables|HitTracing|GetHitArray) (.HitActor (Collision|BreakHitResult _array_element)))
        ;[1 0.1424 0.856] Impact Particle
        (Effects|SpawnEmitteratLocation "/Game/Art/Particles/P_PunchImpact.P_PunchImpact" (LocalVariables|GetLocalSocketlocation) "0.000000,0.000000,0.000000")
        ;[1 0.8473 0.1357] Audio
        (Utilities|FlowControl|DoOnce false :!label _label
          (:Completed
            (Class|AkGameplayStatics|PostEvent (Variables|Default|GetPunchImpactSound) (Class|BaseWeapon|GetPawnOwner) true)
            ;[1 0.1972 0] Set Firing Forcefeedback
            (if (Utilities|IsValid _returnvalue)
              (bind _asplayer_controller (Utilities|Casting|CastToPlayerController (Pawn|GetController _returnvalue)))
              (Game|Feedback|ClientPlayForceFeedback _asplayer_controller "/Game/Blueprints/ForceFeedback/Firing/FFE_Firing_Punch.FFE_Firing_Punch" false "Firing"))))))
    (:Completed
      (goto _label Reset))))

(fn GetControllerforCharacter
  (bind _returnvalue (Class|BaseWeapon|GetPawnOwner))
  (Utilities|IsValid _returnvalue
    (:Is%20Valid
      (bind _asplayer_controller (Utilities|Casting|CastToPlayerController (Pawn|GetController _returnvalue))
        (:then
          (bind _output_get (Variables|Default|SetPlayerController _asplayer_controller))
          (return _output_get))
        (:CastFailed
          _)))
    (:Is%20Not%20Valid
      _))
  (return 0))