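; BP_ZAP is a charge-up weapon that fires only once its charge is full.
; Starting an attack begins charging and caps the owner's walk speed, while stopping restores the saved speed.
; Tick moves the charge toward maximum or back down at a constant rate.
; AttackWithWeapon resets a full charge, stops charging, broadcasts recoil and calls the parent attack; client attack simulation also requires full charge.
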(event EventOnStartAttacking
  ;[1 1 1] Charging states
  (if true
    (CallFunction|StartCharging)))

(event EventOnStopAttacking
  ;[1 1 1] Charging states
  (CallFunction|StopCharging))

(event EventClientSimulateWeaponAttack
  (if (>= (Variables|Default|GetcurrentCharge) (Variables|Default|GetmaxCharge))
    (|CallParentFunction)))

(event EventTick
  (params (DeltaSeconds :type Float%20%28single-precision%29))
  (bind _chargespeed (Variables|Default|GetchargeSpeed))
  ;[1 1 1] Charge and un-charge
  (if (Variables|Default|GetisCharging)
    (Variables|Default|SetcurrentCharge (Math|Interpolation|FInterptoConstant (Variables|Default|GetcurrentCharge) (Variables|Default|GetmaxCharge) DeltaSeconds _chargespeed))
    (else
      (Variables|Default|SetcurrentCharge (Math|Interpolation|FInterptoConstant (Variables|Default|GetcurrentCharge) 0.0 DeltaSeconds _chargespeed)))))

(fn ConstructionScript)

(fn AttackwithWeapon
  (if (Variables|Default|GetisCharging)
    (if (>= (Variables|Default|GetcurrentCharge) (Variables|Default|GetmaxCharge))
      (Variables|Default|SetcurrentCharge 0.0)
      (CallFunction|StopCharging)
      (Class|BaseWeapon|BroadcastonWeaponFiredwithRecoil (.RecoilAmount (Utilities|Struct|BreakRangedWeaponSpreadConfig (Variables|Default|GetSpreadConfig))))
      (bind _returnvalue (|CallParentFunction))
      (return _returnvalue)
      (else
        _)))
  (return false))

(fn StartCharging
  (bind _returnvalue (Class|BaseWeapon|GetPawnOwner))
  (bind _charactermovement (Variables|/Script/Engine.Character|GetCharacterMovement _returnvalue))
  (Variables|Default|SetisCharging true)
  (if (Utilities|IsValid _returnvalue)
    (Variables|Default|SetsavedMaxMoveSpeed (Variables|/Script/Engine.CharacterMovementComponent|GetMaxWalkSpeed _charactermovement))
    (Variables|/Script/Engine.CharacterMovementComponent|SetMaxWalkSpeed _charactermovement (Variables|Default|GetmaxMoveSteedWhilstCharging))))

(fn StopCharging
  (bind _returnvalue (Class|BaseWeapon|GetPawnOwner))
  (Variables|Default|SetisCharging false)
  (if (Utilities|IsValid _returnvalue)
    (Variables|/Script/Engine.CharacterMovementComponent|SetMaxWalkSpeed (Variables|/Script/Engine.Character|GetCharacterMovement _returnvalue) (Variables|Default|GetsavedMaxMoveSpeed))))