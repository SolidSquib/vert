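; BP_GetDamageType translates a damage type class into its matching enum value.
; WhichDamageType compares the class by exact equality down a branch chain covering weapon, melee, thrown, radial and player pod damage types.
; Each match sets the enum and converges on a shared return, while unmatched classes, including subclasses of listed types, have no explicit fallback value.
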(fn WhichDamageType
  (params (DamageTypeClass :type Damage%20Type%20Class%20Reference))
  (if (== DamageTypeClass "/Game/Blueprints/Weapons/DamageTypes/DamageTaken/BP_DamageType_Taken_Chaingun.BP_DamageType_Taken_Chaingun_C")
    (LocalVariables|SetEnum "NewEnumerator0")
    (return (LocalVariables|GetEnum))
    (elif (== DamageTypeClass "/Game/Blueprints/Weapons/DamageTypes/DamageTaken/BP_DamageType_Taken_Shotgun.BP_DamageType_Taken_Shotgun_C")
      (LocalVariables|SetEnum "NewEnumerator1")
      (return (LocalVariables|GetEnum))
      (elif (== DamageTypeClass "/Game/Blueprints/Weapons/DamageTypes/DamageTaken/BP_DamageType_Taken_Buckshot.BP_DamageType_Taken_Buckshot_C")
        (LocalVariables|SetEnum "NewEnumerator5")
        (return (LocalVariables|GetEnum))
        (elif (== DamageTypeClass "/Game/Blueprints/Weapons/DamageTypes/DamageTaken/BP_DamageType_Taken_ForgeHammer.BP_DamageType_Taken_ForgeHammer_C")
          (LocalVariables|SetEnum "NewEnumerator3")
          (return (LocalVariables|GetEnum))
          (elif (== DamageTypeClass "/Game/Blueprints/Weapons/DamageTypes/DamageTaken/BP_DamageType_Taken_Punch.BP_DamageType_Taken_Punch_C")
            (LocalVariables|SetEnum "NewEnumerator4")
            (return (LocalVariables|GetEnum))
            (elif (== DamageTypeClass "/Game/Blueprints/Weapons/DamageTypes/DamageTaken/BP_DamageType_Taken_ZAP.BP_DamageType_Taken_ZAP_C")
              (LocalVariables|SetEnum "NewEnumerator2")
              (return (LocalVariables|GetEnum))
              (elif (== DamageTypeClass "/Game/Blueprints/Weapons/DamageTypes/DamageTaken/BP_DamageType_Thrown.BP_DamageType_Thrown_C")
                (LocalVariables|SetEnum "NewEnumerator13")
                (return (LocalVariables|GetEnum))
                (elif (== DamageTypeClass "/Game/Blueprints/Weapons/DamageTypes/DamageTaken/BP_DamageType_Taken_Radial.BP_DamageType_Taken_Radial_C")
                  (LocalVariables|SetEnum "NewEnumerator11")
                  (return (LocalVariables|GetEnum))
                  (elif (== DamageTypeClass "/Game/Blueprints/Weapons/DamageTypes/DamageTaken/BP_DamageType_Taken_PlayerPod.BP_DamageType_Taken_PlayerPod_C")
                    (LocalVariables|SetEnum "NewEnumerator12")
                    (return (LocalVariables|GetEnum))))))))))))