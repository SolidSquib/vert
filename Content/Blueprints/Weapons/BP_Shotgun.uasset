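; Shotgun weapon Blueprint that fires several pellets per shot by repeating the parent attack in AttackWithWeapon, then posts a Wwise fire sound.
; Starting an attack requires WeaponReady, clears it, calls the parent logic and WeaponAttackFire, and plays controller force feedback for player owners.
; In live code only WeaponReadyfromPickup sets WeaponReady again; an older delay-based refire chain is left disconnected.
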(event EventBeginPlay)

(event Collision|EventActorBeginOverlap
  (params (OtherActor :type Actor%20Object%20Reference)))

(event EventWeaponReadyfromPickup
  (Variables|Default|SetWeaponReady true))

(event EventTick
  (params (DeltaSeconds :type Float%20%28single-precision%29)))

(event EventOnStartAttacking
  (bind _returnvalue (Class|BaseWeapon|GetPawnOwner))
  (if (Variables|Default|GetWeaponReady)
    (Variables|Default|SetWeaponReady false)
    (|CallParentFunction)
    (Class|BaseWeapon|WeaponAttackFire 1.0)
    ;[1 0.1972 0] Set Firing Forcefeedback
    (if (Utilities|IsValid _returnvalue)
      (bind _asplayer_controller (Utilities|Casting|CastToPlayerController (Pawn|GetController _returnvalue)))
      (Game|Feedback|ClientPlayForceFeedback _asplayer_controller "/Game/Blueprints/ForceFeedback/Firing/FFE_Firing_Shotgun.FFE_Firing_Shotgun" false "Firing"))))

(event EventOnStopAttacking
  (params (forced :type Boolean)))

(fn ConstructionScript)

(fn AttackwithWeapon
  (bind _firesound (Variables|Default|GetFireSound))
  (for _index (range 0 (Variables|Default|GetAmountOfBullets))
    (|CallParentFunction))
  (Utilities|IsValid _firesound
    (:Is%20Valid
      (Class|AkGameplayStatics|PostEvent _firesound (Class|BaseWeapon|GetPawnOwner) true))
    (:Is%20Not%20Valid
      _))
  (return true))