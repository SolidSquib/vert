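; Player-steered pod targeting laser that slides along X with MoveRight input, easing toward an interpolated target.
; Each tick it traces down through its position and draws a pulsing debug line in the owning player's armour colour.
; A spawned TopActor follows the floor hit or trace end, and both actors register with VertGameMode as follow targets.
; CheckForVisibleFloorHit returns the first hit regardless of render state, leaving its skip-and-retrace logic unreached.
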(event EventBeginPlay
  (Utilities|FlowControl|Sequence
    (:then_0
      (bind _asvert_game_mode (Utilities|Casting|CastToVertGameMode (Game|GetGameMode)))
      (bind _output_get (Variables|Helper|SetVertGameMode _asvert_game_mode))
      (Class|VertGameMode|RegisterActortoFollow _output_get self)
      (bind _asplayer_controller (Utilities|Casting|CastToPlayerController (Components|GetOwner)))
      (bind _output_get_2 (Variables|Member|SetPlayerController _asplayer_controller))
      (Utilities|IsValid _output_get_2
        (:Is%20Valid
          (bind _asvert_player_state (Utilities|Casting|CastToVertPlayerState (Variables|/Script/Engine.Controller|GetPlayerState _asplayer_controller)))
          (Variables|Member|SetLineColour (.ArmourColour (Utilities|Struct|BreakPlayerColours (Class|VertPlayerState|GetPlayerColours _asvert_player_state))))
          (Variables|Member|SetInterpTarget (Transformation|GetActorLocation)))))
    (:then_1
      (bind _returnvalue (Game|SpawnActorfromClass "/Script/Engine.Actor" (Transformation|GetActorTransform) "AlwaysSpawn" 0 0))
      (Variables|Helper|SetTopActor _returnvalue)
      (Utilities|IsValid (Variables|Helper|GetVertGameMode)
        (:Is%20Valid
          (Class|VertGameMode|RegisterActortoFollow (Variables|Helper|GetVertGameMode) _returnvalue))))))

(event EventTick
  (params (DeltaSeconds :type Float%20%28single-precision%29))
  (bind _returnvalue (Transformation|GetActorLocation))
  (bind _returnvalue_2 (Transformation|GetActorLocation))
  (bind _returnvalue_3 (Transformation|GetActorLocation))
  (bind _topactor (Variables|Helper|GetTopActor))
  (bind _vertgamemode (Variables|Helper|GetVertGameMode))
  (bind _linecolour (Variables|Member|GetLineColour))
  (bind (_x _y _z) (Math|Vector|BreakVector _returnvalue))
  (bind (_x_2 _y_2) (Math|Vector|BreakVector _returnvalue_2))
  (bind (_x_3 _y_3) (Math|Vector|BreakVector _returnvalue_3))
  (bind _returnvalue_4 (+ _z 2e+03))
  (bind _returnvalue_5 (Math|Vector|MakeVector _x _y _returnvalue_4))
  (bind (_x_4 _y_4 _z_2) (Math|Vector|BreakVector _returnvalue_5))
  (bind _returnvalue_6 (- _z_2 4e+03))
  (bind _returnvalue_7 (Math|Vector|MakeVector _x_4 _y_4 _returnvalue_6))
  (Variables|Member|SetRunningTime (+ DeltaSeconds (Variables|Member|GetRunningTime)))
  (Utilities|FlowControl|Sequence
    (:then_0
      (Utilities|IsValid _vertgamemode
        (:Is%20Valid
          (Utilities|IsValid (Class|VertGameMode|GetActivePlayerCamera _vertgamemode)
            (:Is%20Valid
              (bind (_visiblefloorfound _visiblefloorlocation) (CallFunction|CheckforVisibleFloorHit _returnvalue_5 _returnvalue_7))
              (if _visiblefloorfound
                (Rendering|Debug|DrawDebugLine _returnvalue_5 _visiblefloorlocation _linecolour 0.0 (stale _output_get))
                (Transformation|SetActorLocation _topactor (Math|Vector|MakeVector _x_2 _y_2 (.Z (Math|Vector|BreakVector _visiblefloorlocation))) false true)
                (else
                  (Rendering|Debug|DrawDebugLine _returnvalue_5 _returnvalue_7 _linecolour 0.0 (stale _output_get))
                  (Transformation|SetActorLocation _topactor (Math|Vector|MakeVector _x_3 _y_3 (.Z (Math|Vector|BreakVector _returnvalue_7))) false true))))))))
    (:then_1
      (bind _output_get (Variables|Member|SetLaserThickness (+ 16.0 (* (- (Math|Trig|Sin(Radians) (Variables|Member|GetRunningTime)) 0.0) (Variables|Member|GetThicknessModifier))))))
    (:then_2
      (Transformation|SetActorLocation (Math|Interpolation|VInterpTo (Transformation|GetActorLocation) (Variables|Member|GetInterpTarget) (Utilities|Time|GetWorldDeltaSeconds) (Variables|Member|GetInterpSpeed)) false false))))

(event EventEndPlay
  (params (EndPlayReason :type EEndPlayReason%20Enum :default "Destroyed"))
  (bind _vertgamemode (Variables|Helper|GetVertGameMode))
  (bind _topactor (Variables|Helper|GetTopActor))
  (Class|VertGameMode|UnregisterActortoFollow _vertgamemode self)
  (Utilities|IsValid _topactor
    (:Is%20Valid
      (Class|VertGameMode|UnregisterActortoFollow _vertgamemode _topactor)
      (Actor|DestroyActor _topactor))))

(event EventMoveRight
  (params (value :type Float%20%28single-precision%29))
  (Variables|Member|SetInterpTarget (Math|Vector|MakeVector (+ (* (Variables|Member|GetMovementSpeed) (* (Utilities|Time|GetWorldDeltaSeconds) value)) (.X (Math|Vector|BreakVector (Variables|Member|GetInterpTarget)))) (.Y (Math|Vector|BreakVector (Variables|Member|GetInterpTarget))) (.Z (Math|Vector|BreakVector (Variables|Member|GetInterpTarget))))))

(fn ConstructionScript)

(fn CheckforVisibleFloorHit
  (params (TraceStart :type Vector) (TraceEnd :type Vector))
  (bind _output_get (LocalVariables|SetLocalTraceStart TraceStart))
  (while (not (LocalVariables|GetBreakLoop))
    (bind (_outhit _returnvalue) (Collision|LineTraceByChannel _output_get TraceEnd "TraceTypeQuery1" false (LocalVariables|GetIgnoreActors) "None"))
    (if _returnvalue
      (if (Utilities|IsValid (.HitActor (Collision|BreakHitResult _outhit)))
        (if (Class|Actor|WasRecentlyRendered (.HitActor (Collision|BreakHitResult _outhit)) 1.0)
          _
          (else
            _))
        (return true (.ImpactPoint (Collision|BreakHitResult _outhit)))
        (else
          (return true (.ImpactPoint (Collision|BreakHitResult _outhit)))))
      (else
        (return false "0, 0, 0"))))
  (return false "0, 0, 0"))