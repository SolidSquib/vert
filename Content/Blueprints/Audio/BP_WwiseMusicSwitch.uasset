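; Trigger volume actor that changes a Wwise switch, presumably for music going by its name, when the active player camera enters it.
; On overlap it checks that the overlapping actor is the camera from VertGameMode, then sets the configured switch group and value on the game mode actor.
; The SwitchTriggered flag gates the change but is never set in this graph, so the switch can fire on every entry.
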(event OnComponentBeginOverlap(TriggerVolume)
  (params (OverlappedComponent :type Primitive%20Component%20Object%20Reference) (OtherActor :type Actor%20Object%20Reference) (OtherComp :type Primitive%20Component%20Object%20Reference) (OtherBodyIndex :type Integer) (bFromSweep :type Boolean) (SweepResult :type Hit%20Result%20Structure%20%28by%20ref%29))
  (bind _asvert_game_mode (Utilities|Casting|CastToVertGameMode (Game|GetGameMode)))
  (if (and (not (Variables|Default|GetSwitchTriggered)) (== (Class|VertGameMode|GetActivePlayerCamera _asvert_game_mode) OtherActor))
    (Class|AkGameplayStatics|SetSwitch (Variables|Default|GetSwitchGroup) (Variables|Default|GetSwitchValue) _asvert_game_mode)))

(event EventBeginPlay)

(event Collision|EventActorBeginOverlap
  (params (OtherActor :type Actor%20Object%20Reference)))

(event EventTick
  (params (DeltaSeconds :type Float%20%28single-precision%29)))

(fn ConstructionScript)