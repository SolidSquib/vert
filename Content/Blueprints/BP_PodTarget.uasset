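; BP_PodTarget is a player-owned pod target marker that slides along the world X axis, shown with a particle effect in that player's colour.
; On BeginPlay it seeds its goal at its spawn location, then tints all four spawner colours with the owning VertPlayerController's primary player colour.
; MoveRight shifts the goal by frame-time-scaled input, and Tick eases the actor towards it with VInterpTo for smoothed motion.
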(event EventBeginPlay
  (bind _targetparticleeffect (Variables|Default|GetTargetParticleEffect))
  (Variables|Default|SetInterpTarget (Transformation|GetActorLocation))
  (bind _asvert_player_controller (Utilities|Casting|CastToVertPlayerController (Components|GetOwner)))
  (bind _asvert_player_state (Utilities|Casting|CastToVertPlayerState (Variables|/Script/Engine.Controller|GetPlayerState _asvert_player_controller)))
  (Effects|Components|ParticleSystem|SetColorParameter _targetparticleeffect "Spawner_Col0" (.PrimaryColour (Utilities|Struct|BreakPlayerColours (Class|VertPlayerState|GetPlayerColours _asvert_player_state))))
  (Effects|Components|ParticleSystem|SetColorParameter _targetparticleeffect "Spawner_Col1" (.PrimaryColour (Utilities|Struct|BreakPlayerColours (Class|VertPlayerState|GetPlayerColours _asvert_player_state))))
  (Effects|Components|ParticleSystem|SetColorParameter _targetparticleeffect "Spawner_Col2" (.PrimaryColour (Utilities|Struct|BreakPlayerColours (Class|VertPlayerState|GetPlayerColours _asvert_player_state))))
  (Effects|Components|ParticleSystem|SetColorParameter _targetparticleeffect "Spawner_Col3" (.PrimaryColour (Utilities|Struct|BreakPlayerColours (Class|VertPlayerState|GetPlayerColours _asvert_player_state)))))

(event EventTick
  (params (DeltaSeconds :type Float%20%28single-precision%29))
  (Transformation|SetActorLocation (Math|Interpolation|VInterpTo (Transformation|GetActorLocation) (Variables|Default|GetInterpTarget) DeltaSeconds (Variables|Default|GetInterpSpeed)) false false))

(event EventMoveRight
  (params (value :type Float%20%28single-precision%29))
  (Variables|Default|SetInterpTarget (Math|Vector|MakeVector (+ (* (Variables|Default|GetMovementSpeed) (* (Utilities|Time|GetWorldDeltaSeconds) value)) (.X (Math|Vector|BreakVector (Variables|Default|GetInterpTarget)))) (.Y (Math|Vector|BreakVector (Variables|Default|GetInterpTarget))) (.Z (Math|Vector|BreakVector (Variables|Default|GetInterpTarget))))))

(fn ConstructionScript)