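; BP_Elevator is an interactive elevator that starts rising only once every player in the session is inside its collision volume.
; Overlap begin and end events keep a player count, compared against the GameState PlayerArray length, with debug prints while waiting or when someone leaves.
; When the counts match, it latches a started flag, calls CallElevatorMoving and plays a timeline that offsets the mesh's relative Z, stopped after a delay.
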(event OnComponentBeginOverlap(Collision)
  (params (OverlappedComponent :type Primitive%20Component%20Object%20Reference) (OtherActor :type Actor%20Object%20Reference) (OtherComp :type Primitive%20Component%20Object%20Reference) (OtherBodyIndex :type Integer) (bFromSweep :type Boolean) (SweepResult :type Hit%20Result%20Structure%20%28by%20ref%29))
  (if (not (Variables|Default|GetStarted%20Moving))
    (Utilities|FlowControl|Sequence
      (:then_0
        (Variables|Default|SetPlayers (Utilities|Array|Length (Variables|/Script/Engine.GameStateBase|GetPlayerArray (Game|GetGameState))))
        (Variables|Default|SetElevatorMovement (Variables|/Script/Engine.SceneComponent|GetRelativeLocation (Variables|Default|GetSM_Elevator))))
      (:then_1
        (Variables|Default|SetNumberOfPlayers (+ (Variables|Default|GetNumberOfPlayers) 1))
        (Math|Integer|CompareInt (Variables|Default|GetNumberOfPlayers) (Variables|Default|GetPlayers)
          (:==
            (Variables|Default|SetStarted%20Moving true)
            (Default|CallElevatorMoving)
            (bind _floatingisland_01_timeline (Timeline|Timeline_0 Play)
              (:Update
                (Transformation|SetRelativeLocation (Variables|Default|GetSM_Elevator) (+ (Math|Vector|MakeVector 0.0 0.0 _floatingisland_01_timeline) (Variables|Default|GetElevatorMovement)) false false)
                (Utilities|FlowControl|Delay 8.0)
                (Timeline|Timeline_0 Stop))))
          (:<
            (Development|PrintString "Not Enough People")))))))

(event OnComponentEndOverlap(Collision)
  (params (OverlappedComponent :type Primitive%20Component%20Object%20Reference) (OtherActor :type Actor%20Object%20Reference) (OtherComp :type Primitive%20Component%20Object%20Reference) (OtherBodyIndex :type Integer))
  (Variables|Default|SetNumberOfPlayers (- (Variables|Default|GetNumberOfPlayers) 1))
  (Development|PrintString "Player left volume"))

(fn ConstructionScript)