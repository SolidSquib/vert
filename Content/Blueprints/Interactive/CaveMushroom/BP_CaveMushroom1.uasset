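; BP_CaveMushroom1 is a cave mushroom bounce pad that launches characters upward, with a growing risk of exploding instead.
; A capsule trigger tracks overlapping characters, and Tick rolls RNG against the current chance whenever it is occupied and unlocked.
; A hit deals radial damage with knockback, spawns particles and destroys the actor.
; A miss raises the chance, flags the AnimBP's spring, launches occupants after a delay, then unlocks after a cooldown.
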(event OnComponentEndOverlap(Collision_Capsule_Launcher)
  (params (OverlappedComponent :type Primitive%20Component%20Object%20Reference) (OtherActor :type Actor%20Object%20Reference) (OtherComp :type Primitive%20Component%20Object%20Reference) (OtherBodyIndex :type Integer))
  (Utilities|Casting|CastToCharacter OtherActor)
  (Utilities|Array|RemoveItem (Variables|Default|GetOverlappingActors) OtherActor))

(event OnComponentBeginOverlap(Collision_Capsule_Launcher)
  (params (OverlappedComponent :type Primitive%20Component%20Object%20Reference) (OtherActor :type Actor%20Object%20Reference) (OtherComp :type Primitive%20Component%20Object%20Reference) (OtherBodyIndex :type Integer) (bFromSweep :type Boolean) (SweepResult :type Hit%20Result%20Structure%20%28by%20ref%29))
  (Utilities|Casting|CastToCharacter OtherActor)
  (if (== (Utilities|Array|FindItem (Variables|Default|GetOverlappingActors) OtherActor) -1)
    (Utilities|Array|AddUnique (Variables|Default|GetOverlappingActors) OtherActor)))

(event EventBeginPlay
  (bind _asbp_cave_mushroom_animation (Utilities|Casting|CastToBP_CaveMushroomAnimation (Components|SkeletalMesh|GetAnimInstance (Variables|Default|GetSK_CaveMushroom_0)))
    (:then
      (Variables|Default|SetBP_CaveMushroomAnimation _asbp_cave_mushroom_animation)
      (Development|PrintString "Mushroom Cast Successful"))
    (:CastFailed
      (Development|PrintString "Mushroom Cast Failed"))))

(event Collision|EventActorBeginOverlap
  (params (OtherActor :type Actor%20Object%20Reference)))

(event EventTick
  (params (DeltaSeconds :type Float%20%28single-precision%29))
  (if (not (Variables|Default|GetIsLocked))
    ;[1 1 1] Are there any overlapping players that need to be launched?
    (if (> (Utilities|Array|Length (Variables|Default|GetOverlappingActors)) 0)
      (bind _triggered (CallFunction|RNG (Variables|Default|GetCurrentChance)))
      (if _triggered
        (Class|VertUtilities|VERTApplyRadialDamage self (Variables|Default|GetRadialDamage) (Variables|Default|GetRadialKnockback) 1.0 0.0 (Transformation|GetSocketLocation (Variables|Default|GetSK_CaveMushroom_0) "LaunchSocket") 1e+02 "/Game/Blueprints/Weapons/DamageTypes/DamageTaken/BP_DamageType_Taken_Radial.BP_DamageType_Taken_Radial_C" (Utilities|Array|MakeArray (Components|GetOwner)) self 0 true "ECC_Visibility")
        (Effects|SpawnEmitteratLocation "/Game/Art/Particles/P_PlayerDeath.P_PlayerDeath" (Transformation|GetSocketLocation (Variables|Default|GetSK_CaveMushroom_0) "LaunchSocket"))
        (Actor|DestroyActor)
        (else
          (Variables|Default|SetCurrentChance (+ (Variables|Default|GetCurrentChance) (Variables|Default|GetIncrementChance)))
          ;[1 1 1] The Spring animation and Launch force
          ;;[1 1 1] Start the Mushroom animation and stop it from being called again
          (Variables|/Game/Blueprints/Interactive/CaveMushroom/BP_CaveMushroomAnimation.BP_CaveMushroomAnimation_C|SetIsSpringing (Variables|Default|GetBP_CaveMushroomAnimation) true)
          (Variables|Default|SetIsLocked true)
          (Utilities|FlowControl|Delay (Variables|Default|GetSpringLaunchDelay))
          (bind _array_element (Utilities|Array|ForEachLoopwithBreak (Variables|Default|GetOverlappingActors))
            (:LoopBody
              (bind _ascharacter (Utilities|Casting|CastToCharacter _array_element))
              (Character|LaunchCharacter _ascharacter "0, 0,2000.000000" false true))
            (:Completed
              ;;[1 1 1] How long before the Mushroom will activate again
              (Utilities|FlowControl|Delay (Variables|Default|GetSpringCooldown))
              (Variables|Default|SetIsLocked false))))))))

(fn ConstructionScript)