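; Prototype shared-camera actor that keeps two BP_VertCharacter characters framed together.
; On BeginPlay it becomes the view target for player controllers 0 to 3 and caches the first two characters found.
; Each Tick it moves to their midpoint and sets the camera arm length to their separation, so the view zooms as they spread.
; Without a valid second character, it follows the first and leaves the arm length unchanged.
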(event EventBeginPlay
  (for _array_element (Utilities|Array|MakeArray (Game|GetPlayerController 0) (Game|GetPlayerController 1) (Game|GetPlayerController 2) (Game|GetPlayerController 3))
    (Game|Player|SetViewTargetwithBlend _array_element self 0.0 "VTBlend_Linear" 0.0 false)
    ;[1 1 1] Store refferences to both characters in variables
    (bind _outactors (Actor|GetAllActorsOfClass "/Game/Blueprints/Characters/BP_VertCharacter.BP_VertCharacter_C"))
    (Variables|Default|SetC1 (Utilities|Array|Get(acopy) _outactors))
    (Variables|Default|SetC2 (Utilities|Array|Get(acopy) _outactors 1))))

(event EventTick
  (params (DeltaSeconds :type Float%20%28single-precision%29))
  (bind _c2 (Variables|Default|GetC2))
  (Utilities|IsValid _c2
    (:Is%20Valid
      ;[1 1 1] Distance between two actors
      (Variables|Default|SetDistance (- (Transformation|GetActorLocation (Variables|Default|GetC1)) (Transformation|GetActorLocation _c2)))
      (Utilities|FlowControl|Sequence
        (:then_0
          ;[1 1 1] Update the position of the CamerFocusActor and adjust the Camera Arm Length
          (Transformation|SetActorLocation (+ (Transformation|GetActorLocation (Variables|Default|GetC2)) (/ (Variables|Default|GetDistance) 2.0)) false false)
          (Variables|/Script/Engine.SpringArmComponent|SetTargetArmLength (Variables|Default|GetCamera%20Arm) (Math|Vector|VectorLength (Variables|Default|GetDistance))))))
    (:Is%20Not%20Valid
      (Transformation|SetActorLocation (Transformation|GetActorLocation (Variables|Default|GetC1)) false false))))

(fn ConstructionScript)