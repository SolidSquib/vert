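; Player drop pod pawn that delivers a player into the level, with respawn audio, controller rumble and radial impact damage on landing.
; Charging rumble starts from a timeline on spawn; the pod's initial-velocity event stops rumble and audio and hides the flame.
; Tick traces downward to place a floor target, which is tinted with the beam's dynamic materials to the possessing player's colour.
; Projectile stop halts mesh rotation; stops and overlaps trigger impact effects and force feedback.
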(event OnProjectileStop(ProjectileMovement)
  (params (ImpactResult :type Hit%20Result%20Structure%20%28by%20ref%29))
  (bind _returnvalue (Components|GetOwner))
  (bind _returnvalue_2 (Pawn|GetController))
  (bind _self self)
  (bind _rotatingmovement (Variables|Default|GetRotatingMovement))
  (Utilities|FlowControl|Sequence
    (:then_0
      (Components|Movement|StopMovementImmediately _rotatingmovement)
      (Components|Movement|SetUpdatedComponent _rotatingmovement 0))
    (:then_1
      ;[1 0.1424 0.856] Spawn Ground Impact FX
      (Effects|SpawnEmitteratLocation "/Game/Art/Particles/P_HammerImpact.P_HammerImpact" (Transformation|GetSocketLocation (Variables|Character|GetMesh) "Thruster_Socket")))
    (:then_2
      (bind _asplayer_controller (Utilities|Casting|CastToPlayerController _returnvalue))
      (Class|VertUtilities|VERTApplyRadialDamage _self 2e+01 3e+01 1.0 0.1 (Transformation|GetSocketLocation (Variables|Character|GetMesh) "Thruster_Socket") 2e+02 "/Game/Blueprints/Weapons/DamageTypes/DamageTaken/BP_DamageType_Taken_PlayerPod.BP_DamageType_Taken_PlayerPod_C" (Utilities|Array|MakeArray _returnvalue) _self _asplayer_controller true "ECC_Visibility"))
    (:then_3
      ;[1 0.1972 0] Apply ForceFeedback to owner if they hit a player (Might need changing to make sure its just players)
      (if (Utilities|IsValid _returnvalue_2)
        (bind _asplayer_controller_2 (Utilities|Casting|CastToPlayerController _returnvalue_2))
        (Game|Feedback|ClientPlayForceFeedback _asplayer_controller_2 "/Game/Blueprints/ForceFeedback/Firing/FFE_Firing_Forgehammer.FFE_Firing_Forgehammer" false "Firing")))))

(event EventBeginPlay
  (bind _returnvalue (Pawn|GetController))
  (Utilities|FlowControl|Sequence
    (:then_0
      (Components|Timeline|SetPlayRate (Variables|Default|GetPodChargingForceFeedback) 3.0)
      (bind _blend_chargestrength (Timeline|PodChargingForceFeedback PlayFromStart)
        (:Update
          ;[1 0.1972 0] Set Charging Forcefeedback
          (if (Utilities|IsValid _returnvalue)
            (bind _asplayer_controller (Utilities|Casting|CastToPlayerController _returnvalue))
            (Game|Feedback|PlayDynamicForceFeedback _asplayer_controller (Math|Float|Lerp 0.0 0.3 _blend_chargestrength) -1.0 false true false true)))))
    (:then_1
      (for (_array_element _array_index) (Rendering|Material|GetMaterials (Variables|Default|GetSMBeam))
        (bind _returnvalue_2 (Rendering|Material|CreateDynamicMaterialInstance (Variables|Default|GetSMBeam) _array_index _array_element :!class /Script/Engine.PrimitiveComponent))
        (Utilities|Array|Add (Variables|Default|GetDynamicMIDS) _returnvalue_2)))
    (:then_2
      (Class|AkGameplayStatics|PostEvent "/Game/WwiseAudio/Player/Re_Spawn.Re_Spawn" self false))))

(event EventOnPodInitVelocity
  (Utilities|FlowControl|Sequence
    (:then_0
      (Rendering|SetVisibility (Variables|Default|GetDroppodFlame) false true))
    (:then_1
      ;[1 0.1972 0] Set Charging Forcefeedback
      (Game|Feedback|PlayDynamicForceFeedback (stale EventBeginPlay _asplayer_controller) (Math|Float|Lerp 0.0 0.3 (stale EventBeginPlay _blend_chargestrength)) -1.0 false true false true) ; enters at Stop
    )
    (:then_2
      (Class|AkGameplayStatics|PostEvent "/Game/WwiseAudio/Player/Re_Spawn_Stop.Re_Spawn_Stop" self false))))

(event EventPossessed
  (params (NewController :type Controller%20Object%20Reference))
  (CallFunction|SetColour NewController))

(event EventOnPodOverlap
  (params (overlappedComponent :type Primitive%20Component%20Object%20Reference) (otherActor :type Actor%20Object%20Reference) (otherComp :type Primitive%20Component%20Object%20Reference) (otherBodyIndex :type Integer) (fromSweep :type Boolean) (sweepResult :type Hit%20Result%20Structure%20%28by%20ref%29))
  (bind _returnvalue (Components|GetOwner))
  (|CallParentFunction overlappedComponent otherActor otherComp otherBodyIndex fromSweep sweepResult)
  (Utilities|FlowControl|Sequence
    (:then_0
      ;[1 0.1972 0] Apply ForceFeedback to owner if they hit a player (Might need changing to make sure its just players)
      (if (Utilities|IsValid _returnvalue)
        (bind _asplayer_controller (Utilities|Casting|CastToPlayerController _returnvalue))
        (Game|Feedback|ClientPlayForceFeedback _asplayer_controller "/Game/Blueprints/ForceFeedback/Firing/FFE_Firing_Forgehammer.FFE_Firing_Forgehammer" false "Firing")))
    (:then_1
      (Effects|SpawnEmitteratLocation "/Game/Art/Particles/P_HammerImpact.P_HammerImpact" (Transformation|GetSocketLocation (Variables|Character|GetMesh) "Thruster_Socket")))))

(event EventTick
  (params (DeltaSeconds :type Float%20%28single-precision%29))
  (bind _returnvalue (Transformation|GetActorLocation))
  (bind _floortarget (Variables|Default|GetFloorTarget))
  (bind (_x _y _z) (Math|Vector|BreakVector _returnvalue))
  (bind _returnvalue_2 (- _z 5e+03))
  (bind _returnvalue_3 (Math|Vector|MakeVector _x _y _returnvalue_2))
  (bind (_outhit _returnvalue_4) (Collision|LineTraceForObjects _returnvalue _returnvalue_3 (Utilities|Array|MakeArray "ObjectTypeQuery1") false 0 "None"))
  (if _returnvalue_4
    (Transformation|SetWorldLocation _floortarget (.ImpactPoint (Collision|BreakHitResult _outhit)) false false)
    (else
      (Transformation|SetWorldLocation _floortarget _returnvalue_3 false false))))

(fn ConstructionScript
  (Components|Movement|SetUpdatedComponent (Variables|Default|GetRotatingMovement) (Variables|Character|GetMesh)))

(fn SetColour
  (params (New%20Controller :type Controller%20Object%20Reference))
  (bind _floortarget (Variables|Default|GetFloorTarget))
  (bind _asvert_player_controller (Utilities|Casting|CastToVertPlayerController New%20Controller))
  (bind _asvert_player_state (Utilities|Casting|CastToVertPlayerState (Variables|/Script/Engine.Controller|GetPlayerState _asvert_player_controller)))
  (for _array_element (Variables|Default|GetDynamicMIDS)
    (Rendering|Material|SetVectorParameterValue _array_element "Col" (.PrimaryColour (Utilities|Struct|BreakPlayerColours (Class|VertPlayerState|GetPlayerColours _asvert_player_state))) :!class /Script/Engine.MaterialInstanceDynamic)
    (Effects|Components|ParticleSystem|SetColorParameter _floortarget "Spawner_Col0" (.PrimaryColour (Utilities|Struct|BreakPlayerColours (Class|VertPlayerState|GetPlayerColours _asvert_player_state))))
    (Effects|Components|ParticleSystem|SetColorParameter _floortarget "Spawner_Col1" (.PrimaryColour (Utilities|Struct|BreakPlayerColours (Class|VertPlayerState|GetPlayerColours _asvert_player_state))))
    (Effects|Components|ParticleSystem|SetColorParameter _floortarget "Spawner_Col2" (.PrimaryColour (Utilities|Struct|BreakPlayerColours (Class|VertPlayerState|GetPlayerColours _asvert_player_state))))
    (Effects|Components|ParticleSystem|SetColorParameter _floortarget "Spawner_Col3" (.PrimaryColour (Utilities|Struct|BreakPlayerColours (Class|VertPlayerState|GetPlayerColours _asvert_player_state))))))