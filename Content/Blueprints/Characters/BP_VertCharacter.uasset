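; Character Blueprint that handles ledge grabbing and records action states such as jump, dash, attack, grapple, item pickup and weapon state, with debug prints.
; While airborne inside a LedgeTracer overlap, forward and downward sphere traces find the wall and ledge.
; A one-time trigger switches movement to Flying and moves the capsule to the edge.
; Landing velocity drives a timeline-blended animation strength, reversed when running along X.
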(event OnComponentBeginOverlap(LedgeTracer)
  (params (OverlappedComponent :type Primitive%20Component%20Object%20Reference) (OtherActor :type Actor%20Object%20Reference) (OtherComp :type Primitive%20Component%20Object%20Reference) (OtherBodyIndex :type Integer) (bFromSweep :type Boolean) (SweepResult :type Hit%20Result%20Structure%20%28by%20ref%29))
  ;[1 1 1] OnComponentOverlap LedgeTracer
  (Variables|Michael|SetCanTrace true)
  (Development|PrintString "Hello"))

(event OnComponentEndOverlap(LedgeTracer)
  (params (OverlappedComponent :type Primitive%20Component%20Object%20Reference) (OtherActor :type Actor%20Object%20Reference) (OtherComp :type Primitive%20Component%20Object%20Reference) (OtherBodyIndex :type Integer))
  ;[1 1 1] OnComponentOverlap LedgeTracer
  (Variables|Michael|SetCanTrace false)
  (Development|PrintString "goodbye"))

(event Custom|CEvent%20%20OnJumpApex
  ;[0.9301 0.5711 1] OnJumpApex Event - Set IsJumping False
  (Variables|LocomotionState|SetIsJumping? false))

(event EventCharacteronInteractExecuted
  (params (interactive :type Interactive%20Object%20Reference))
  ;[1 0.187 0.177] On Interact / Attack
  ;[1 1 1] Debugging
  (Development|PrintString "OnInteract" false))

(event EventCharacteronGrappleShootExecuted
  (params (direction :type Vector%20%28by%20ref%29))
  ;[0.3989 0.9101 1] On Grapple Shoot / Pull
  (bind _output_get (Variables|UserInput|SetGrappleDirection direction))
  ;[1 1 1] Debugging
  (Development|PrintString (Utilities|String|ToString(Vector) _output_get) false))

(event EventCharacteronGrapplePullExecuted
  (params (direction :type Vector%20%28by%20ref%29 :default "0, 0, 0"))
  ;[0.3989 0.9101 1] On Grapple Shoot / Pull
)

(event EventCharacteronDropCurrentInteractive
  (params (interactive :type Interactive%20Object%20Reference) (wasThrown :type Boolean))
  ;[1 0.9156 0.9057] Pickup / Drop Interactives
  (Variables|WeaponInteract|SetItem_PickedUp false)
  (Variables|WeaponInteract|SetItem_Dropped true)
  ;[1 1 1] Debugging
  (Development|PrintString "OnDropCurrent" false))

(event EventCharacteronDashExecuted
  (params (direction :type Vector%20%28by%20ref%29 :default "0, 0, 0") (isGrappled :type Boolean))
  ;[0.2999 1 0.496] On Dash Start / End
  (Variables|UserInput|SetDashButton_IsDown true))

(event EventOnLanded
  (params (Hit :type Hit%20Result%20Structure%20%28by%20ref%29))
  ;[0.9301 0.5711 1] OnLanded Event - Set OnLandedVelocity
  (bind _output_get (Variables|LandValues|SetOnLandedVelocity (Math|Float|NormalizetoRange (.Z (Math|Vector|BreakVector (Variables|/Script/Engine.MovementComponent|GetVelocity (Variables|Character|GetCharacterMovement)))) 0.0 3e+03)))
  (Development|PrintString (Utilities|String|ToString(Float) _output_get) false)
  ;[0.54 0.4266 0.08657] Play AnimationBlend Timeline - Set CrouchStrengthBlend
  (bind _animationblend (Timeline|Land%20Smooth%20Blend%20Timeline PlayFromStart)
    (:Update
      (Variables|LandValues|SetAnimationBlend_LandStrength (Math|Float|Lerp 0.0 (* (Variables|LandValues|GetOnLandedVelocity) -1.0) _animationblend))
      (bind _isrunning (CallFunction|IsRunning?))
      (if _isrunning
        (Utilities|FlowControl|DoOnce false :!label _label
          (:Completed
            (Timeline|Land%20Smooth%20Blend%20Timeline Reverse)))
        (else
          (goto _label Reset))))))

(event EventCharacteronDashEnded
  ;[0.2999 1 0.496] On Dash Start / End
  (Variables|UserInput|SetDashButton_IsDown false))

(event EventTick
  (params (DeltaSeconds :type Float%20%28single-precision%29))
  (bind _returnvalue (Transformation|GetActorLocation))
  (bind _returnvalue_2 (Transformation|GetActorRotation))
  (bind _returnvalue_3 (Transformation|GetActorLocation))
  (bind _returnvalue_4 (Transformation|GetActorRotation))
  (bind _capsulecomponent (Variables|Default|GetCapsuleComponent))
  (bind (_x _y _z) (Math|Vector|BreakVector _returnvalue))
  (bind _returnvalue_5 (Math|Vector|GetForwardVector _returnvalue_2))
  (bind (_x_2 _y_2 _z_2) (Math|Vector|BreakVector _returnvalue_3))
  (bind _returnvalue_6 (Math|Vector|GetForwardVector _returnvalue_4))
  (bind _capsuleradius (Variables|/Script/Engine.CapsuleComponent|GetCapsuleRadius _capsulecomponent))
  (bind _returnvalue_7 (- _z_2 0.0))
  (bind (_x_3 _y_3 _z_3) (Math|Vector|BreakVector _returnvalue_6))
  (bind _returnvalue_8 (* _returnvalue_5 7e+01))
  (bind _returnvalue_9 (+ _z 5e+02))
  (bind _returnvalue_10 (Math|Vector|MakeVector _x _y _returnvalue_9))
  (bind _returnvalue_11 (Math|Vector|MakeVector _x_2 _y_2 _returnvalue_7))
  (bind _returnvalue_12 (+ _returnvalue_10 _returnvalue_8))
  (bind (_x_4 _y_4 _z_4) (Math|Vector|BreakVector _returnvalue_12))
  (Utilities|FlowControl|Sequence
    (:then_0
      (if (and (Variables|Michael|GetCanTrace) (not (Class|VertCharacter|IsGrounded)))
        (Utilities|FlowControl|Sequence
          (:then_0
            (bind (_outhit _returnvalue_13) (Collision|SphereTraceByChannel _returnvalue_11 (+ _returnvalue_11 (Math|Vector|MakeVector (* _x_3 1.5e+02) (* _y_3 1.5e+02) (- _z_3 0.0))) 2e+01 "TraceTypeQuery3" false (Utilities|Array|MakeArray 0) "ForOneFrame"))
            (if _returnvalue_13
              (Variables|Michael|SetWallTraceImpact (.ImpactPoint (Collision|BreakHitResult _outhit)))
              (Variables|Michael|SetWallNormal (.ImpactNormal (Collision|BreakHitResult _outhit)))))
          (:then_1
            (if _returnvalue_13
              (bind (_outhit_2 _returnvalue_14) (Collision|SphereTraceByChannel _returnvalue_12 (Math|Vector|MakeVector _x_4 _y_4 (- _z_4 5.5e+02)) 2e+01 "TraceTypeQuery3" false (Utilities|Array|MakeArray 0) "ForOneFrame"))
              (if _returnvalue_14
                (Variables|Michael|SetLedge%20Height (.ImpactPoint (Collision|BreakHitResult _outhit_2)))
                (Utilities|FlowControl|DoOnce false
                  (:Completed
                    (if (not (Variables|LocomotionState|GetIsClimbingLedge))
                      (Pawn|Components|CharacterMovement|SetMovementMode (Variables|Character|GetCharacterMovement) "MOVE_Flying" 0)
                      (Components|MoveComponentTo (Variables|Default|GetCapsuleComponent) (Math|Vector|MakeVector (+ (.X (Math|Vector|BreakVector (* (Variables|Michael|GetWallNormal) (Math|Vector|MakeVector _capsuleradius _capsuleradius 0.0)))) (.X (Math|Vector|BreakVector (Variables|Michael|GetWallTraceImpact)))) (+ (.Y (Math|Vector|BreakVector (* (Variables|Michael|GetWallNormal) (Math|Vector|MakeVector _capsuleradius _capsuleradius 0.0)))) (.Y (Math|Vector|BreakVector (Variables|Michael|GetWallTraceImpact)))) (- (.Z (Math|Vector|BreakVector (Variables|Michael|GetLedge%20Height))) (Components|Capsule|GetScaledCapsuleHalfHeight _capsulecomponent))) (Math|Rotator|FindLookatRotation (Transformation|GetActorLocation) (Variables|Michael|GetWallTraceImpact)) false false 0.2 false)
                      (Components|Movement|StopMovementImmediately (Variables|Character|GetCharacterMovement)))))))))))))

(event EventBeginPlay
  ;[0.9301 0.5711 1] OnJumpApex Event - Set IsJumping False
  (Variables|/Script/Engine.CharacterMovementComponent|SetbNotifyApex (Variables|Character|GetCharacterMovement) true)
  (EventDispatchers|BindEventtoOnReachedJumpApex (delegate Custom|CEvent%20%20OnJumpApex)))

(event EventCharacteronJumpExecuted
  ;[0.9301 0.5711 1] OnJump Event - Set IsJumping True
  (Variables|LocomotionState|SetIsJumping? true))

(event EventCharacteronStopAttackExecuted
  ;[1 0.187 0.177] On Interact / Attack
  (Variables|UserInput|SetAttackButton_IsDown false)
  ;[1 1 1] Debugging
  (Development|PrintString "AttackbuttonIsDown: False" false))

(event EventCharacteronStartAttackExecuted
  (params (weapon :type Base%20Weapon%20Object%20Reference))
  ;[1 0.187 0.177] On Interact / Attack
  (Variables|UserInput|SetAttackButton_IsDown true)
  ;[1 1 1] Debugging
  (Development|PrintString "AttackButtonIsDown: True" false))

(event EventCharacteronPickupNewInteractive
  (params (interactive :type Interactive%20Object%20Reference) (wasCaught :type Boolean))
  ;[1 0.9156 0.9057] Pickup / Drop Interactives
  (Variables|WeaponInteract|SetItem_Dropped false)
  (Variables|WeaponInteract|SetItem_PickedUp true)
  ;[1 1 1] Debugging
  (Development|PrintString "OnPickupNew" false))

(event EventCharacteronWeaponStateChangeExecuted
  (params (weapon :type Base%20Weapon%20Object%20Reference) (newState :type EWeaponState%20Enum :default "Idle") (playerAnim :type Anim%20Sequence%20Object%20Reference))
  ;[1 0.187 0.177] On Interact / Attack
  ;[1 1 1] Debugging
  (Development|PrintString "WeaponStateChange Executed" false false)
  (CallFunction|SetWeaponStates weapon newState playerAnim))

(event EventCharacteronWeaponFiredwithRecoilExecuted
  (params (recoilAmount :type Float%20%28single-precision%29))
  ;[1 0.187 0.177] On Interact / Attack
  ;[1 1 1] Debugging
  (Development|PrintString "WeaponFired With Recoil" false))

(fn ConstructionScript)

(fn IsRunning?
  (bind _returnvalue (Transformation|GetVelocity))
  (bind _x (Math|Vector|BreakVector _returnvalue))
  (return (or (> _x 1e+01) (< _x -1e+01))))

(fn SetWeaponStates
  (params (NewWeaponReference :type Base%20Weapon%20Object%20Reference) (NewWeaponState :type EWeaponState%20Enum) (NewAnimation :type Anim%20Sequence%20Object%20Reference))
  (bind _output_get (Variables|WeaponState|SetECurrentWeaponState NewWeaponState))
  (bind _output_get_2 (Variables|WeaponState|SetECurrentWeaponAnimation NewAnimation))
  (Variables|WeaponState|SetCurrentWeaponReference NewWeaponReference)
  ;[1 1 1] Debugging Output
  (Development|PrintString (Utilities|String|ToString(Text) (Utilities|Text|FormatText "Weapon State: {WeaponState}" (Utilities|Text|ToText(String) (Utilities|String|EnumtoString _output_get)))))
  (Development|PrintString (Utilities|String|ToString(Text) (Utilities|Text|FormatText "Weapon Animation Mode: {WeaponAnimationMode}" (Utilities|Text|ToText(String) (Utilities|GetDisplayName _output_get_2))))))