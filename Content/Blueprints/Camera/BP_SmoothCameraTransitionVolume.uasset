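; Camera transition volume that delays its transition until the active camera reaches the end of its track.
; CameraOverlapped ignores inactive cameras and runs the parent transition logic only when ShouldTransition is set, otherwise binding to the camera's end-of-track event.
; OnReachedEndOfTrack sets the flag and re-runs CameraOverlapped, and nothing here clears the flag afterward.
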(fn ConstructionScript)

(fn CameraOverlapped
  (params (camera :type Vert%20Player%20Camera%20Actor%20Object%20Reference))
  (if (Class|VertPlayerCameraActor|IsCameraActive camera)
    (if (Variables|Default|GetShouldTransition)
      (bind _returnvalue (|CallParentFunction camera))
      (return _returnvalue)
      (else
        (EventDispatchers|BindEventtoOnCameraReachEndOfTrack camera (EventDispatchers|CreateEvent :!event OnReachedEndOfTrack))
        (return false)))))

(fn OnReachedEndOfTrack
  (params (Camera :type Vert%20Player%20Camera%20Actor%20Object%20Reference))
  (Variables|Default|SetShouldTransition true)
  (CallFunction|CameraOverlapped Camera))