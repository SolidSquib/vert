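; Base game mode Blueprint that adds a sudden death finale and crowd audio reactions to player kills.
; When the finale starts, it creates a scrolling sudden death widget whose countdown expiry disables player respawns.
; Player kills post Wwise events: a boo for AI killers, applause for player killers.
; Each sound has its own short cooldown, decremented on Tick, to limit repeats.
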(event Custom|Start%20Sudden%20Death
  (Class|VertGameMode|SetCanPlayersRespawn false))

(event EventTick
  (params (DeltaSeconds :type Float%20%28single-precision%29))
  (Utilities|FlowControl|Sequence
    (:then_0
      (if (> (Variables|Default|GetBoo%20Cooldown) 0.0)
        (Variables|Default|SetBoo%20Cooldown (- (Variables|Default|GetBoo%20Cooldown) DeltaSeconds))))
    (:then_1
      (if (> (Variables|Default|GetCheer%20Cooldown) 0.0)
        (Variables|Default|SetCheer%20Cooldown (- (Variables|Default|GetCheer%20Cooldown) DeltaSeconds))))))

(event EventHandleFinaleHasStarted
  (|CallParentFunction)
  (bind _returnvalue (UserInterface|CreateWidget "/Game/UI/HUD/UIW_SuddenDeath.UIW_SuddenDeath_C"))
  (Utilities|IsValid _returnvalue
    (:Is%20Valid
      (Default|StartScrolling _returnvalue)
      (EventDispatchers|BindEventtoOnTimerExpired (Variables|/Game/UI/HUD/UIW_SuddenDeath.UIW_SuddenDeath_C|GetUIW_SuddenDeathCountdown _returnvalue) (delegate Custom|Start%20Sudden%20Death)))))

(event EventOnPlayerKilled
  (params (Killer :type Controller%20Object%20Reference) (KilledPawn :type Pawn%20Object%20Reference))
  (Utilities|FlowControl|Sequence
    (:then_0
      (Utilities|Casting|CastToAIController Killer)
      (if (<= (Variables|Default|GetBoo%20Cooldown) 0.0)
        (Class|AkGameplayStatics|PostEvent "/Game/WwiseAudio/Audience/Boo.Boo" self false)
        (Variables|Default|SetBoo%20Cooldown 5.0)))
    (:then_1
      (Utilities|Casting|CastToPlayerController Killer)
      (if (<= (Variables|Default|GetCheer%20Cooldown) 0.0)
        (Class|AkGameplayStatics|PostEvent "/Game/WwiseAudio/Audience/Crowd_Applause.Crowd_Applause" self false)
        (Variables|Default|SetCheer%20Cooldown 5.0)))))

(fn ConstructionScript)