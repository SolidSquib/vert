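; Player drop pod, a child Blueprint that adds player colour, effects, rumble and landing damage to its parent pod.
; On BeginPlay it tints the beam through dynamic materials using the owning player's primary colour, and a timeline drives a ramping charge rumble.
; Initial velocity hides the flame and stops that rumble; impact stops rotation.
; Overlaps and hits spawn impact effects and owner feedback, with hits also dealing radial damage and knockback, sparing the owner.
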(event EventBeginPlay
  (bind _returnvalue (Components|GetOwner))
  (Utilities|FlowControl|Sequence
    (:then_0
      (for (_array_element _array_index) (Rendering|Material|GetMaterials (Variables|Default|GetSM_Beam))
        (bind _returnvalue_2 (Rendering|Material|CreateDynamicMaterialInstance (Variables|Default|GetSM_Beam) _array_index _array_element :!class /Script/Engine.PrimitiveComponent))
        (Utilities|Array|Add (Variables|Default|GetDynamicMIDS) _returnvalue_2)))
    (:then_1
      (CallFunction|SetColour))
    (:then_2
      (Components|Timeline|SetPlayRate (Variables|Default|GetPodChargingForceFeedback) 3.0)
      (bind _blend_chargestrength (Timeline|PodChargingForceFeedback PlayFromStart)
        (:Update
          ;[1 0.1972 0] Set Charging Forcefeedback
          (if (Utilities|IsValid _returnvalue)
            (bind _asplayer_controller (Utilities|Casting|CastToPlayerController _returnvalue))
            (Game|Feedback|PlayDynamicForceFeedback _asplayer_controller (Math|Float|Lerp 0.0 0.3 _blend_chargestrength) -1.0 false true false true)))))))

(event EventOnPodMadeImpact
  (bind _rotatingmovement (Variables|Default|GetRotatingMovement))
  (Components|Movement|StopMovementImmediately _rotatingmovement)
  (Components|Activation|Deactivate _rotatingmovement))

(event EventOnPodInitVelocity
  (Utilities|FlowControl|Sequence
    (:then_0
      (Rendering|SetVisibility (Variables|Default|GetP_DroppodFlame) false true))
    (:then_1
      ;[1 0.1972 0] Set Charging Forcefeedback
      (Game|Feedback|PlayDynamicForceFeedback (stale EventBeginPlay _asplayer_controller) (Math|Float|Lerp 0.0 0.3 (stale EventBeginPlay _blend_chargestrength)) -1.0 false true false true) ; enters at Stop
    )))

(event EventOnPodOverlap
  (params (overlappedComponent :type Primitive%20Component%20Object%20Reference) (otherActor :type Actor%20Object%20Reference) (otherComp :type Primitive%20Component%20Object%20Reference) (otherBodyIndex :type Integer) (fromSweep :type Boolean) (sweepResult :type Hit%20Result%20Structure%20%28by%20ref%29))
  (bind _returnvalue (Components|GetOwner))
  (|CallParentFunction overlappedComponent otherActor otherComp otherBodyIndex fromSweep sweepResult)
  (Utilities|FlowControl|Sequence
    (:then_0
      ;[1 0.1972 0] Apply ForceFeedback to owner if they hit a player (Might need changing to make sure its just players)
      (if (Utilities|IsValid _returnvalue)
        (bind _asplayer_controller (Utilities|Casting|CastToPlayerController _returnvalue))
        (Game|Feedback|ClientPlayForceFeedback _asplayer_controller "/Game/Blueprints/ForceFeedback/Firing/FFE_Firing_Forgehammer.FFE_Firing_Forgehammer" false "Firing")))
    (:then_1
      (Effects|SpawnEmitteratLocation "/Game/Art/Particles/P_HammerImpact.P_HammerImpact" (Transformation|GetSocketLocation (Variables|Default|GetMeshComponent) "Thruster_Socket")))))

(event EventOnPodHit
  (params (hit :type Hit%20Result%20Structure%20%28by%20ref%29))
  (bind _returnvalue (Components|GetOwner))
  (bind _returnvalue_2 (Components|GetOwner))
  (bind _self self)
  (|CallParentFunction hit)
  (Utilities|FlowControl|Sequence
    (:then_0
      (bind _asplayer_controller (Utilities|Casting|CastToPlayerController _returnvalue_2))
      (Class|VertUtilities|VERTApplyRadialDamage _self 2e+01 3e+01 1.0 0.1 (Transformation|GetSocketLocation (Variables|Default|GetMeshComponent) "Thruster_Socket") 2e+02 "/Game/Blueprints/Weapons/DamageTypes/DamageTaken/BP_DamageType_Taken_Radial.BP_DamageType_Taken_Radial_C" (Utilities|Array|MakeArray _returnvalue_2) _self _asplayer_controller true "ECC_Visibility"))
    (:then_1
      ;[1 0.1424 0.856] Spawn Ground Impact FX
      (Effects|SpawnEmitteratLocation "/Game/Art/Particles/P_HammerImpact.P_HammerImpact" (Transformation|GetSocketLocation (Variables|Default|GetMeshComponent) "Thruster_Socket")))
    (:then_2
      ;[1 0.1972 0] Apply ForceFeedback to owner if they hit a player (Might need changing to make sure its just players)
      (if (Utilities|IsValid _returnvalue)
        (bind _asplayer_controller_2 (Utilities|Casting|CastToPlayerController _returnvalue))
        (Game|Feedback|ClientPlayForceFeedback _asplayer_controller_2 "/Game/Blueprints/ForceFeedback/Firing/FFE_Firing_Forgehammer.FFE_Firing_Forgehammer" false "Firing")))))

(fn ConstructionScript
  (|CallParentFunction))

(fn SetColour
  (Utilities|FlowControl|Sequence
    (:then_0
      (bind _asvert_player_controller (Utilities|Casting|CastToVertPlayerController (Components|GetOwner)))
      (bind _asvert_player_state (Utilities|Casting|CastToVertPlayerState (Variables|/Script/Engine.Controller|GetPlayerState _asvert_player_controller)))
      (for _array_element (Variables|Default|GetDynamicMIDS)
        (Rendering|Material|SetVectorParameterValue _array_element "Col" (.PrimaryColour (Utilities|Struct|BreakPlayerColours (Class|VertPlayerState|GetPlayerColours _asvert_player_state))) :!class /Script/Engine.MaterialInstanceDynamic)))))