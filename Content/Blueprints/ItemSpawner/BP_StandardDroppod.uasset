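; BP_StandardDroppod is a drop pod in the item spawner system that plays a ground impact effect when it lands.
; When the pooled pod begins play it starts a two-second safety timer, which disables and destroys it if it expires.
; On impact it clears that timer and spawns a hammer impact emitter at the mesh's thruster socket.
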(event Custom|OnSafetyTimerEnd
  (Class|DropPod|DisableandDestroy))

(event EventEVENTonPoolBeginPlay
  (bind _returnvalue (Utilities|Time|SetTimerbyEvent (delegate Custom|OnSafetyTimerEnd) 2.0))
  (Variables|Default|SetSafety%20Timer _returnvalue))

(event EventOnPodMadeImpact
  (Utilities|FlowControl|Sequence
    (:then_0
      (Utilities|Time|ClearandInvalidateTimerbyHandle (Variables|Default|GetSafety%20Timer)))
    (:then_1
      ;[1 0.1424 0.856] Spawn Ground Impact FX
      (Effects|SpawnEmitteratLocation "/Game/Art/Particles/P_HammerImpact.P_HammerImpact" (Transformation|GetSocketLocation (Variables|Default|GetMeshComponent) "Thruster_Socket")))))

(fn ConstructionScript)